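; Stats actor component for the inventory system, with DELETE-prefixed names, storing values such as health, stamina, armor and damage in a map.
; Server events route add, remove and set to authority-only functions that clamp values and notify the client, which updates its map and broadcasts changes.
; Health and Stamina are capped by their max stats, re-checked after removes and sets.
; Initialization binds to owner equipment events, but item-stat functions are empty.
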(event Custom|DELETE_Server%20Add%20Stat%20Value
  (params (Stat :type EStatCategory%20Enum :default "None") (Value :type Float%20%28double-precision%29))
  ;[0.1198 0.1198 0.1198 0.525] Server Events
  (CallFunction|DELETEAddStatValue Stat Value))

(event Custom|DELETE_Server%20Remove%20Stat%20Value
  (params (Stat :type EStatCategory%20Enum :default "None") (Value :type Float%20%28double-precision%29))
  ;[0.1198 0.1198 0.1198 0.525] Server Events
  (CallFunction|DELETERemoveStatValue Stat Value))

(event Custom|DELETE_Server%20Set%20Stat%20Value
  (params (Stat :type EStatCategory%20Enum :default "None") (Value :type Float%20%28double-precision%29))
  ;[0.1198 0.1198 0.1198 0.525] Server Events
  (CallFunction|DELETESetStatValue Stat Value))

(event Custom|DELETE_Client%20Stat%20Value%20Changed
  (params (Stat :type EStatCategory%20Enum :default "None") (Stat%20Value :type Float%20%28double-precision%29))
  ;[0.1198 0.1198 0.1198 0.525] Client Events
  (Utilities|Map|Add (Variables|Default|GetStats) Stat Stat%20Value)
  (Default|CallOnChangedStatValue Stat Stat%20Value))

(event Custom|DELETE_Initialize%20Stats
  ;[1 0 0.04033 0.587] Initialize Stats Component [Event called from Owner]
  (CallFunction|DELETEClientInitializeStats))

(event Custom|DELETE_Client%20Initialize%20Stats
  (bind _returnvalue (Components|GetOwner))
  (bind _returnvalue_2 (Actor|GetComponentbyClass _returnvalue "/Game/InventorySystem/Blueprints/Components/DELETE_AC_PlayerEquipment.DELETE_AC_PlayerEquipment_C"))
  ;[1 0.01447 0 0.561] CLIENT: Initialize Stats Component
  (Default|CallOnRefreshStats)
  (Utilities|IsValid _returnvalue_2
    (:Is%20Valid
      (Variables|Default|SetOwner%20Equipment _returnvalue_2)
      (EventDispatchers|BindEventtoOnAddedtoEquipment (Variables|Default|GetOwner%20Equipment) (EventDispatchers|CreateEvent :!event DELETEAddItemStats))
      (EventDispatchers|BindEventtoOnRemovedfromEquipment (Variables|Default|GetOwner%20Equipment) (EventDispatchers|CreateEvent :!event DELETERemoveItemStats)))))

(fn DELETEAddStatValue
  (params (Stat :type EStatCategory%20Enum :default "None") (Value :type Float%20%28double-precision%29))
  (bind _stats (Variables|Default|GetStats))
  (bind (_value _returnvalue) (Utilities|Map|Find _stats Stat))
  (Utilities|DELETESwitchHasOwnerAuthority
    (:Authority
      (if _returnvalue
        (Utilities|Map|Add (Variables|Default|GetStats) Stat (CallFunction|DELETEClampStatValue Stat (+ _value Value)))
        (CallFunction|DELETEClientStatValueChanged Stat (.Value (Utilities|Map|Find (Variables|Default|GetStats) Stat)))))))

(fn DELETEGetStatValue
  (params (Stat :type EStatCategory%20Enum :default "None"))
  (bind _stats (Variables|Default|GetStats))
  (bind (_value _returnvalue) (Utilities|Map|Find _stats Stat))
  (if _returnvalue
    (return _value)
    (else
      (return 0.0))))

(fn DELETEClampStatValue
  (params (Stat :type EStatCategory%20Enum :default "None") (Value :type Float%20%28double-precision%29))
  (if (or (Utilities|Enum|Equal(Enum) Stat "Health") (Utilities|Enum|Equal(Enum) Stat "Stamina"))
    (return (Math|Float|Clamp(Float) Value 0.0 (Utilities|Select :Index Stat :None 0.0 :Health (CallFunction|DELETEGetStatValue "MaxHealth") :MaxHealth 0.0 :Stamina (CallFunction|DELETEGetStatValue "MaxStamina") :MaxStamina 0.0 :Armor 0.0 :Damage 0.0 :AttackSpeed 0.0)))
    (else
      (return (Math|Float|Clamp(Float) Value 0.0 Value)))))

(fn DELETERemoveStatValue
  (params (Stat :type EStatCategory%20Enum :default "None") (Value :type Float%20%28double-precision%29))
  (bind _stats (Variables|Default|GetStats))
  (bind (_value _returnvalue) (Utilities|Map|Find _stats Stat))
  (Utilities|DELETESwitchHasOwnerAuthority
    (:Authority
      (if _returnvalue
        (Utilities|Map|Add (Variables|Default|GetStats) Stat (CallFunction|DELETEClampStatValue Stat (- _value Value)))
        (CallFunction|DELETEClientStatValueChanged Stat (.Value (Utilities|Map|Find (Variables|Default|GetStats) Stat)))
        (CallFunction|DELETEFixAnyMiscalculations)))))

(fn DELETEAddItemStats
  (params (Item%20Data :type DELETE%20S%20Item%20Data%20Structure)))

(fn DELETERemoveItemStats
  (params (Item%20Data :type DELETE%20S%20Item%20Data%20Structure)))

(fn DELETESetStatValue
  (params (Stat :type EStatCategory%20Enum :default "None") (Value :type Float%20%28double-precision%29))
  (Utilities|DELETESwitchHasOwnerAuthority
    (:Authority
      (if (.ReturnValue (Utilities|Map|Find (Variables|Default|GetStats) Stat))
        (Utilities|Map|Add (Variables|Default|GetStats) Stat (CallFunction|DELETEClampStatValue Stat Value))
        (CallFunction|DELETEClientStatValueChanged Stat (.Value (Utilities|Map|Find (Variables|Default|GetStats) Stat)))
        (CallFunction|DELETEFixAnyMiscalculations)))))

(fn DELETEFixAnyMiscalculations
  (for _array_element (Utilities|Array|MakeArray "Health" "Stamina")
    (LocalVariables|SetL%20Stat _array_element)
    (if (> (CallFunction|DELETEGetStatValue _array_element) (CallFunction|DELETEGetStatValue (Utilities|Select :Index _array_element :None "None" :Health "MaxHealth" :MaxHealth "None" :Stamina "MaxStamina" :MaxStamina "None" :Armor "None" :Damage "None" :AttackSpeed "None")))
      (Utilities|Map|Add (Variables|Default|GetStats) (LocalVariables|GetL%20Stat) (CallFunction|DELETEClampStatValue (LocalVariables|GetL%20Stat) (CallFunction|DELETEGetStatValue (Utilities|Select :Index _array_element :None "None" :Health "MaxHealth" :MaxHealth "None" :Stamina "MaxStamina" :MaxStamina "None" :Armor "None" :Damage "None" :AttackSpeed "None"))))
      (CallFunction|DELETEClientStatValueChanged (LocalVariables|GetL%20Stat) (.Value (Utilities|Map|Find (Variables|Default|GetStats) (LocalVariables|GetL%20Stat)))))))

(fn DELETEGetMaxStatValue
  (params (Stat :type EStatCategory%20Enum :default "None"))
  (bind _value (CallFunction|DELETEGetStatValue "MaxStamina"))
  (bind _value_2 (CallFunction|DELETEGetStatValue "MaxHealth"))
  (if (.ReturnValue (Utilities|Map|Find (Variables|Default|GetStats) Stat))
    (return (Utilities|Select :Index Stat :None 0.0 :Health _value_2 :MaxHealth _value_2 :Stamina _value :MaxStamina _value :Armor 999.0 :Damage 999.0 :AttackSpeed 999.0))
    (else
      (return 0.0))))