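; DELETE-prefixed player equipment component on the PlayerController, managing items worn by the RPG character.
; Server-side functions equip, swap, stack and remove items in a slot-keyed map, mirrored to clients by RPCs that fire dispatchers.
; Armor updates character meshes, while weapons and shields spawn as socket-attached actors.
; Equipping from inventory checks level and, with off-hand enabled, resolves one/two-hand conflicts; initial equipment loads from DataTable rows.
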(fn DELETEBuildEquipment
  (bind _enumvalue (|ForEachEItemSlot)
    (:LoopBody
      (if (.ReturnValue (Utilities|Map|Find (Variables|Default|GetEquipment%20Data) _enumvalue))
        (bind _structout (Utilities|Struct|SetmembersinDELETE_S_ItemData (.Value (Utilities|Map|Find (Variables|Default|GetEquipment%20Data) _enumvalue)) _enumvalue true))
        (Utilities|Map|Add (Variables|Default|GetEquipment%20Data) _enumvalue _structout)
        (else
          (bind _structout_2 (Utilities|Struct|SetmembersinDELETE_S_ItemData (LocalVariables|GetL%20Empty%20Data) _enumvalue))
          (Utilities|Map|Add (Variables|Default|GetEquipment%20Data) _enumvalue _structout_2))))))

(fn DELETEBuildInitialEquipment
  (bind _returnvalue (Components|GetOwner))
  (bind _returnvalue_2 (Actor|GetComponentbyClass _returnvalue "/Game/InventorySystem/Blueprints/Components/DELETE_AC_InventoryCore.DELETE_AC_InventoryCore_C"))
  (for _array_element (Variables|Default|GetInitial%20Equipment)
    ;[1 0.163 0 0.138 37] Add single row to Equipment Data
    (bind _returnvalue_3 (Utilities|GetDataTableRow (.DataTable (Utilities|Struct|BreakDataTableRowHandle (.tableandrow _array_element))) (.RowName (Utilities|Struct|BreakDataTableRowHandle (.tableandrow _array_element))))
      (:then
        (bind _structout (Utilities|Struct|SetmembersinDELETE_S_ItemData _returnvalue_3 (Math|Integer|Clamp(Integer) (.quantity _array_element) 1 (.quantity _array_element))))
        (bind _output_get (LocalVariables|SetL%20Item%20Data _structout))
        (bind _in_slot_data (CallFunction|DELETEAssignItemfromEquipmentSlot _output_get))
        (CallFunction|DELETEAddItemtoEquipmentArray (LocalVariables|GetL%20Item%20Data) (Utilities|Struct|BreakDELETE_S_ItemData _in_slot_data))
        (CallFunction|DELETEAttachItemtoEquipment (LocalVariables|GetL%20Item%20Data))
        (Utilities|IsValid _returnvalue_2
          (:Is%20Valid
            (Default|DELETEAddWeighttoInventory _returnvalue_2 (Utilities|DELETECalculateStackedItemWeight (LocalVariables|GetL%20Item%20Data))))))))
  ;[0.8225 1 0 0.18] Clear Data Table Variables on Completed
  (Utilities|Array|Clear (Variables|Default|GetInitial%20Equipment)))

(fn DELETEAddItemtoEquipmentArray
  (params (Item%20Data :type DELETE%20S%20Item%20Data%20Structure%20%28by%20ref%29) (Equipment%20Slot :type EItemSlot%20Enum :default "None"))
  ;[1 0 0.06858 0.493] SERVER: Add Item to Equipment Data
  (Utilities|DELETESwitchHasOwnerAuthority
    (:Authority
      (bind _structout (Utilities|Struct|SetmembersinDELETE_S_ItemData Item%20Data Equipment%20Slot true))
      (Utilities|Map|Add (Variables|Default|GetEquipment%20Data) Equipment%20Slot _structout)
      ;[1 0.9656 0 0.493] IF STANDALONE: Call Event Dispatcher
      (if (Class|KismetSystemLibrary|IsStandalone)
        (Default|CallOnAddedtoEquipment Item%20Data)
        (else
          ;[0.1707 1 0 0.493] CLIENT: Update Item
          (CallFunction|ClientUpdateAddedItem Item%20Data))))))

(fn DELETERemoveItemfromEquipmentArray
  (params (Item%20Data :type DELETE%20S%20Item%20Data%20Structure))
  (bind _equipmentslot (Utilities|Struct|BreakDELETE_S_ItemData Item%20Data))
  ;[1 0 0.06858 0.493] SERVER: Remove Item from Equipment Data
  (Utilities|DELETESwitchHasOwnerAuthority
    (:Authority
      (Utilities|Map|Remove (Variables|Default|GetEquipment%20Data) _equipmentslot)
      (bind _structout (Utilities|Struct|SetmembersinDELETE_S_ItemData (LocalVariables|GetL%20Empty%20Data) _equipmentslot))
      (Utilities|Map|Add (Variables|Default|GetEquipment%20Data) _equipmentslot _structout)
      ;[1 0.9656 0 0.493] IF STANDALONE: Call Event Dispatcher
      (if (Class|KismetSystemLibrary|IsStandalone)
        (Default|CallOnRemovedfromEquipment Item%20Data)
        (else
          ;[0.1707 1 0 0.493] CLIENT: Update Item
          (CallFunction|ClientUpdateRemovedItem Item%20Data))))))

(fn DELETEAddtoStackinEquipment
  (params (Item%20Data :type DELETE%20S%20Item%20Data%20Structure) (Equipment%20Slot :type EItemSlot%20Enum :default "None"))
  (bind _equipment_data (Variables|Default|GetEquipment%20Data))
  (bind (_value _returnvalue) (Utilities|Map|Find _equipment_data Equipment%20Slot))
  (if _returnvalue
    (bind _structout (Utilities|Struct|SetmembersinDELETE_S_ItemData _value (+ (.Quantity (Utilities|Struct|BreakDELETE_S_ItemData _value)) (.Quantity (Utilities|Struct|BreakDELETE_S_ItemData Item%20Data)))))
    (CallFunction|DELETEAddItemtoEquipmentArray _structout (.EquipmentSlot (Utilities|Struct|BreakDELETE_S_ItemData _structout)))))

(fn DELETETrytoAddtoPartialStack
  (params (Item%20Data :type DELETE%20S%20Item%20Data%20Structure))
  (bind _values (Utilities|Map|Values (Variables|Default|GetEquipment%20Data)))
  (bind _slot_index (Utilities|DELETEHasPartialStack? _values Item%20Data)
    (:True
      (CallFunction|DELETEAddtoStackinEquipment Item%20Data (Utilities|Struct|BreakDELETE_S_ItemData (Utilities|Array|Get(acopy) _values _slot_index)))
      (return true))
    (:False
      (return false))))

(fn DELETETransferItemfromInventorytoEquipment
  (params (Item%20Data :type DELETE%20S%20Item%20Data%20Structure) (InSlot%20Data :type DELETE%20S%20Item%20Data%20Structure) (Inventory :type DELETE%20AC%20Inventory%20Core%20Object%20Reference) (Method :type EInputMethod%20Enum :default "RightClick"))
  (LocalVariables|SetL%20Item%20Data Item%20Data)
  (LocalVariables|SetL%20InSlot%20Data InSlot%20Data)
  (if (.Return%20Value (CallFunction|DELETECanItembeEquipped? (LocalVariables|GetL%20Item%20Data)))
    (switch Utilities|FlowControl|Switch|SwitchonEInputMethod Method
      (:RightClick
        ;[1 0 0.04044 0.384] Assign appropriate Item from Slot [Only if InSlot Data was not specified before - On Right Click]
        (bind _in_slot_data (CallFunction|DELETEAssignItemfromEquipmentSlot (LocalVariables|GetL%20Item%20Data)))
        (LocalVariables|SetL%20InSlot%20Data _in_slot_data))
      (:DragAndDrop
        _))
    (Utilities|DELETEIsItemClassValid? (LocalVariables|GetL%20InSlot%20Data) ; Not Valid = Empty
      (:Valid
        (Utilities|DELETEAreItemstheSame? (LocalVariables|GetL%20Item%20Data) (LocalVariables|GetL%20InSlot%20Data)
          (:True
            (Utilities|DELETEAreItemsStackable? (LocalVariables|GetL%20Item%20Data) (LocalVariables|GetL%20InSlot%20Data)
              (:True
                ;[1 0.8785 0 0.488] Stack Items
                (CallFunction|DELETEAddtoStackinEquipment (LocalVariables|GetL%20Item%20Data) (Utilities|Struct|BreakDELETE_S_ItemData (LocalVariables|GetL%20InSlot%20Data)))
                (Default|DELETERemoveItemfromInventoryArray Inventory (LocalVariables|GetL%20Item%20Data))
                (return true ""))
              (:False
                _)))
          (:False
            _))
        ;[1 0 0 0.441] Swap Items
        (CallFunction|DELETERemoveItemfromEquipmentArray (LocalVariables|GetL%20InSlot%20Data))
        (Default|DELETEAddItemtoInventoryArray Inventory (LocalVariables|GetL%20InSlot%20Data) (Utilities|Struct|BreakDELETE_S_ItemData (LocalVariables|GetL%20Item%20Data)))
        (CallFunction|DELETEAddItemtoEquipmentArray (LocalVariables|GetL%20Item%20Data) (Utilities|Struct|BreakDELETE_S_ItemData (LocalVariables|GetL%20InSlot%20Data)))
        (CallFunction|DELETEDetachItemfromEquipment (LocalVariables|GetL%20InSlot%20Data))
        (CallFunction|DELETEAttachItemtoEquipment (LocalVariables|GetL%20Item%20Data))
        (CallFunction|DELETETrytoUnequipAssociatedSlot (LocalVariables|GetL%20Item%20Data) Inventory)
        (return true ""))
      (:Not%20Valid
        ;[0.05725 1 0 0.399] Transfer Item to Empty Slot in Equipment
        (Default|DELETERemoveItemfromInventoryArray Inventory (LocalVariables|GetL%20Item%20Data))
        (CallFunction|DELETEAddItemtoEquipmentArray (LocalVariables|GetL%20Item%20Data) (Utilities|Struct|BreakDELETE_S_ItemData (LocalVariables|GetL%20InSlot%20Data)))
        (CallFunction|DELETEAttachItemtoEquipment (LocalVariables|GetL%20Item%20Data))
        (CallFunction|DELETETrytoUnequipAssociatedSlot (LocalVariables|GetL%20Item%20Data) Inventory)
        (return true "")))
    (else
      (return false (.Failure%20Message (CallFunction|DELETECanItembeEquipped? (LocalVariables|GetL%20Item%20Data)))))))

(fn DELETETransferItemfromEquipmenttoEquipment
  (params (Dragged%20Data :type DELETE%20S%20Item%20Data%20Structure) (InSlot%20Data :type DELETE%20S%20Item%20Data%20Structure))
  (LocalVariables|SetL%20Dragged%20Data Dragged%20Data)
  (bind _output_get (LocalVariables|SetL%20InSlot%20Data InSlot%20Data))
  ;[1 0 0.01364 0.436] Is Slot not Empty?
  (Utilities|DELETEIsItemClassValid? _output_get
    (:Valid
      (CallFunction|DELETERemoveItemfromEquipmentArray (LocalVariables|GetL%20InSlot%20Data))
      (CallFunction|DELETEAddItemtoEquipmentArray Dragged%20Data (Utilities|Struct|BreakDELETE_S_ItemData (LocalVariables|GetL%20InSlot%20Data)))
      (CallFunction|DELETERemoveItemfromEquipmentArray (LocalVariables|GetL%20Dragged%20Data))
      (CallFunction|DELETEAddItemtoEquipmentArray InSlot%20Data (Utilities|Struct|BreakDELETE_S_ItemData (LocalVariables|GetL%20Dragged%20Data)))
      (CallFunction|DELETEAttachItemtoEquipment InSlot%20Data)
      (CallFunction|DELETEAttachItemtoEquipment Dragged%20Data))
    (:Not%20Valid
      (CallFunction|DELETERemoveItemfromEquipmentArray (LocalVariables|GetL%20Dragged%20Data))
      (CallFunction|DELETEDetachItemfromEquipment (LocalVariables|GetL%20Dragged%20Data))
      (CallFunction|DELETEAddItemtoEquipmentArray (LocalVariables|GetL%20Dragged%20Data) (Utilities|Struct|BreakDELETE_S_ItemData (LocalVariables|GetL%20InSlot%20Data)))
      (CallFunction|DELETEAttachItemtoEquipment (LocalVariables|GetL%20Dragged%20Data)))))

(fn DELETEAttachItemtoEquipment
  (params (Item%20Data :type DELETE%20S%20Item%20Data%20Structure))
  (bind (_equipmentslot _class) (Utilities|Struct|BreakDELETE_S_ItemData Item%20Data))
  (Utilities|DELETEIsItemClassValid? Item%20Data
    (:Valid
      (LocalVariables|SetL%20Item%20Slot _equipmentslot)
      (LocalVariables|SetL%20Skeletal (Utilities|GetClassDefaults _class))
      (Utilities|IsValid (Variables|Default|GetOwning%20Character)
        (:Is%20Valid
          (Default|CallOnItemAttach Item%20Data)
          (switch Utilities|FlowControl|Switch|SwitchonEItemSlot (LocalVariables|GetL%20Item%20Slot)
            (:Head
              ;[0.05725 1 0 0.285 22] Attach to Master Pose
              (Default|ServerUpdateEquipmentMesh (Variables|Default|GetOwning%20Character) (LocalVariables|GetL%20Item%20Slot) (LocalVariables|GetL%20Skeletal) :!label _label) ; Called on Server inside RPGInventoryCharacterBP
            )
            (:Gloves
              (goto _label))
            (:Neck
              (goto _label))
            (:ChestPlate
              (goto _label))
            (:Legs
              (goto _label))
            (:Boots
              (goto _label))
            (:Weapon
              ;[1 0.8208 0 0.285 22] Attach to Socket
              (CallFunction|ServerSpawnEquippableActor Item%20Data (Variables|Default|GetOwning%20Character) :!label _label_2))
            (:Shield
              (goto _label_2))))))))

(fn DELETEDetachItemfromEquipment
  (params (Item%20Data :type DELETE%20S%20Item%20Data%20Structure))
  (Utilities|IsValid (Variables|Default|GetOwning%20Character)
    (:Is%20Valid
      (Default|CallOnItemDetach Item%20Data)
      (bind _output_get (LocalVariables|SetL%20Item%20Slot (Utilities|Struct|BreakDELETE_S_ItemData Item%20Data)))
      (switch Utilities|FlowControl|Switch|SwitchonEItemSlot _output_get
        (:Head
          ;[0.05725 1 0 0.285 22] Detach Armor
          (Default|ServerUpdateEquipmentMesh (Variables|Default|GetOwning%20Character) (LocalVariables|GetL%20Item%20Slot) :!label _label))
        (:Gloves
          (goto _label))
        (:Neck
          (goto _label))
        (:ChestPlate
          (goto _label))
        (:Legs
          (goto _label))
        (:Boots
          (goto _label))
        (:Weapon
          ;[1 0.5216 0 0.243 22] Detach Weapon Slot
          (CallFunction|ServerDestroyEquippableActor Item%20Data :!label _label_2))
        (:Shield
          (goto _label_2))))))

(fn DELETERemoveItemQuantity
  (params (Item%20Data :type DELETE%20S%20Item%20Data%20Structure) (Quantity :type Integer))
  (bind _output_get (LocalVariables|SetL%20Item%20Data Item%20Data))
  (Math|Integer|CompareInt (Utilities|Struct|BreakDELETE_S_ItemData _output_get) Quantity
    (:>
      (CallFunction|DELETERemoveItemfromEquipmentArray (LocalVariables|GetL%20Item%20Data))
      (bind _structout (Utilities|Struct|SetmembersinDELETE_S_ItemData (LocalVariables|GetL%20Item%20Data) (- (Utilities|Struct|BreakDELETE_S_ItemData (LocalVariables|GetL%20Item%20Data)) Quantity)))
      (CallFunction|DELETEAddItemtoEquipmentArray _structout (Utilities|Struct|BreakDELETE_S_ItemData _structout)))
    (:==
      (CallFunction|DELETERemoveItemfromEquipmentArray Item%20Data :!label _label)
      (CallFunction|DELETEDetachItemfromEquipment Item%20Data))
    (:<
      (goto _label))))

(fn DELETECanItembeEquipped?
  (params (Item%20Data :type DELETE%20S%20Item%20Data%20Structure))
  (bind _returnvalue (Components|GetOwner))
  (bind _returnvalue_2 (Actor|GetComponentbyClass _returnvalue "/Game/InventorySystem/Blueprints/Components/DELETE_AC_Leveling.DELETE_AC_Leveling_C"))
  (if (and (Utilities|IsValid _returnvalue_2) (select (Variables|Default|GetCheck%20Required%20Item%20Level) (>= (Variables|/Game/InventorySystem/Blueprints/Components/DELETE_AC_Leveling.DELETE_AC_Leveling_C|GetCurrent%20Level _returnvalue_2) (Utilities|GetClassDefaults (Utilities|Struct|BreakDELETE_S_ItemData Item%20Data))) true))
    (return true "")
    (else
      (return false "Higher level required."))))

(fn DELETEGetItembyEquipmentSlot
  (params (Slot :type EItemSlot%20Enum :default "None"))
  (bind _equipment_data (Variables|Default|GetEquipment%20Data))
  (bind (_value _returnvalue) (Utilities|Map|Find _equipment_data Slot))
  (if _returnvalue
    (Utilities|DELETEIsItemClassValid? _value
      (:Valid
        (return true _value))
      (:Not%20Valid
        (return false _value)))
    (else
      (return false ""))))

(fn DELETEGetItembyID
  (params (Item%20ID :type String))
  (bind _values (Utilities|Map|Values (Variables|Default|GetEquipment%20Data)))
  (bind _item (Utilities|DELETEFindItembyID _values Item%20ID)
    (:Found
      (return _item true))
    (:Not%20Found
      (return "" false))))

(fn DELETEGetEquipmentItems
  (bind _values (Utilities|Map|Values (Variables|Default|GetEquipment%20Data)))
  (return _values))

(fn DELETEGetEquippedActorReference
  (params (Slot :type EItemSlot%20Enum :default "None"))
  (bind _equipped_weapon_slot (Variables|Default|GetEquipped%20Weapon%20Slot))
  (bind _equipped_shield_slot (Variables|Default|GetEquipped%20Shield%20Slot))
  (bind _returnvalue (Utilities|Select :Index Slot :None 0 :Head 0 :Gloves 0 :Neck 0 :ChestPlate 0 :Legs 0 :Boots 0 :Weapon _equipped_weapon_slot :Shield _equipped_shield_slot :Pocket1 0 :Pocket2 0 :Pocket3 0 :Pocket4 0 :NewSlot 0))
  (Utilities|IsValid _returnvalue
    (:Is%20Valid
      (return _returnvalue))))

(fn DELETETrytoUnequipAssociatedSlot
  (params (Item%20Data :type DELETE%20S%20Item%20Data%20Structure) (Inventory :type DELETE%20AC%20Inventory%20Core%20Object%20Reference))
  (if (Variables|Default|GetEnable%20Off-Hand)
    (LocalVariables|SetL%20Associated%20Slot (Utilities|Select :Index (Utilities|Struct|BreakDELETE_S_ItemData Item%20Data) :None "None" :Head "None" :Gloves "None" :Neck "None" :ChestPlate "None" :Legs "None" :Boots "None" :Weapon "Shield" :Shield "Weapon" :Pocket1 "None" :Pocket2 "None" :Pocket3 "None" :Pocket4 "None" :NewSlot "None"))
    (switch Utilities|FlowControl|Switch|SwitchonEWeaponType (Utilities|GetClassDefaults (Utilities|Struct|BreakDELETE_S_ItemData Item%20Data))
      (:OneHand
        ;[1 0.07874 0 0.478] Check if Two Hand is in the Associated Slot. If so - Remove it
        (if (.IsValid (CallFunction|DELETEGetItembyEquipmentSlot (LocalVariables|GetL%20Associated%20Slot))) :!label _label
          (if (Utilities|Enum|Equal(Enum) (Utilities|GetClassDefaults (Utilities|Struct|BreakDELETE_S_ItemData (.Item%20Data (CallFunction|DELETEGetItembyEquipmentSlot (LocalVariables|GetL%20Associated%20Slot))))) "TwoHand")
            (bind (_success _failure_message) (Default|DELETETransferItemfromEquipment :self Inventory :Item%20Data (.Item%20Data (CallFunction|DELETEGetItembyEquipmentSlot (LocalVariables|GetL%20Associated%20Slot))) :Sender self))
            (Default|DELETEClientTransferItemReturnValue Inventory _success _failure_message))))
      (:TwoHand
        ;[1 0.3781 0 0.598] Check if anything is in the Shield Slot. If so - Remove it
        (if (.IsValid (CallFunction|DELETEGetItembyEquipmentSlot (LocalVariables|GetL%20Associated%20Slot)))
          (bind (_success_2 _failure_message_2) (Default|DELETETransferItemfromEquipment :self Inventory :Item%20Data (.Item%20Data (CallFunction|DELETEGetItembyEquipmentSlot (LocalVariables|GetL%20Associated%20Slot))) :Sender self))
          (Default|DELETEClientTransferItemReturnValue Inventory _success_2 _failure_message_2)))
      (:OffHand
        (goto _label)))))

(fn DELETEAssignItemfromEquipmentSlot
  (params (Item%20Data :type DELETE%20S%20Item%20Data%20Structure))
  (if (Utilities|Set|Contains (Utilities|Set|MakeSet "Pocket1" "Pocket2" "Pocket3" "Pocket4") (Utilities|Struct|BreakDELETE_S_ItemData Item%20Data))
    ;[1 0.7046 0 0.358] Assign Item from Empty/Default Slot [Consumables]
    (bind _slot (Utilities|DELETEFindEmptyEquipmentSlot (Variables|Default|GetEquipment%20Data) (Utilities|Array|MakeArray "Pocket1" "Pocket2" "Pocket3" "Pocket4") "Pocket1")
      (:Found
        _)
      (:Not%20Found
        _))
    (return (.Item%20Data (CallFunction|DELETEGetItembyEquipmentSlot _slot)))
    (else
      ;[1 0.03104 0 0.608] #Check if Item is a One-Hand [AND Off-Hand is Enabled]
      (if (and (Variables|Default|GetEnable%20Off-Hand) (Utilities|Enum|Equal(Enum) (Utilities|GetClassDefaults (Utilities|Struct|BreakDELETE_S_ItemData Item%20Data)) "OneHand"))
        ;[1 0.03104 0 0.608] #Check if there is already One-Hand Weapon in [Shield]Slot
        (if (not (.IsValid (CallFunction|DELETEGetItembyEquipmentSlot "Shield")))
          ;[1 0.7046 0 0.358] Assign Item from Empty/Default Slot [One-hand]
          (bind _slot_2 (Utilities|DELETEFindEmptyEquipmentSlot (Variables|Default|GetEquipment%20Data) (Utilities|Array|MakeArray "Weapon" "Shield") "Weapon")
            (:Found
              _)
            (:Not%20Found
              _))
          (return (.Item%20Data (CallFunction|DELETEGetItembyEquipmentSlot _slot_2)))
          (else
            ;[0.1261 0 1 0.577] Assign Item from Weapon Slot
            (return (.Item%20Data (CallFunction|DELETEGetItembyEquipmentSlot "Weapon")))))
        (else
          ;[0.1352 1 0 0.379] Assign Item from equal Slot [Default]
          (return (.Item%20Data (CallFunction|DELETEGetItembyEquipmentSlot (Utilities|Struct|BreakDELETE_S_ItemData Item%20Data)))))))))

(fn DELETEAttachEquippedItemtoSocket
  (params (Slot :type EItemSlot%20Enum :default "None") (Socket%20Name :type Name))
  (bind _returnvalue (CallFunction|DELETEGetEquippedActorReference Slot))
  (Utilities|IsValid _returnvalue
    (:Is%20Valid
      (Transformation|AttachComponentToComponent _returnvalue (Variables|/Script/Engine.Character|GetMesh (Variables|Default|GetOwning%20Character)) Socket%20Name "SnapToTarget" "SnapToTarget" "SnapToTarget" false))))

(fn DELETESpawnandAttachEquippableActor
  (params (Item%20Data :type DELETE%20S%20Item%20Data%20Structure) (Owning%20Character :type BP%20RPG%20Inventory%20Character%20Object%20Reference))
  (Utilities|DELETESwitchHasOwnerAuthority
    (:Authority
      (Utilities|DELETEIsItemClassValid? Item%20Data
        (:Valid
          (Utilities|IsValid Owning%20Character
            (:Is%20Valid
              (LocalVariables|SetL%20Equippable 0)
              (switch Utilities|FlowControl|Switch|SwitchonEItemSlot (Utilities|Struct|BreakDELETE_S_ItemData Item%20Data)
                (:Weapon
                  ;[1 0.7202 0 0.52 24] Spawn & Attach Weapon [Main-Hand]
                  (Utilities|IsValid (Variables|Default|GetEquipped%20Weapon%20Slot)
                    (:Is%20Valid
                      (Actor|DestroyActor (Variables|Default|GetEquipped%20Weapon%20Slot)))
                    (:Is%20Not%20Valid
                      _))
                  (bind _returnvalue (Game|SpawnActorfromClass (LocalVariables|GetL%20Equippable) (Transformation|GetActorTransform Owning%20Character) "Undefined" "SelectDefaultAtRuntime" Owning%20Character 0))
                  (bind _output_get (Variables|Default|SetEquipped%20Weapon%20Slot _returnvalue))
                  (Transformation|AttachComponentToComponent _output_get (Variables|/Script/Engine.Character|GetMesh Owning%20Character) (Utilities|Select :Index (Utilities|GetClassDefaults (Utilities|Struct|BreakDELETE_S_ItemData Item%20Data)) :None "main_hand" :OneHand "main_hand" :TwoHand "two_hand" :OffHand "main_hand") "SnapToTarget" "SnapToTarget" "SnapToTarget" false))
                (:Shield
                  ;[1 0.3392 0 0.52 24] Spawn & Attach Shield [Off-Hand]
                  (Utilities|IsValid (Variables|Default|GetEquipped%20Shield%20Slot)
                    (:Is%20Valid
                      (Actor|DestroyActor (Variables|Default|GetEquipped%20Shield%20Slot)))
                    (:Is%20Not%20Valid
                      _))
                  (bind _returnvalue_2 (Game|SpawnActorfromClass (LocalVariables|GetL%20Equippable) (Transformation|GetActorTransform Owning%20Character) "Undefined" "SelectDefaultAtRuntime" Owning%20Character 0))
                  (bind _output_get_2 (Variables|Default|SetEquipped%20Shield%20Slot _returnvalue_2))
                  (Transformation|AttachComponentToComponent _output_get_2 (Variables|/Script/Engine.Character|GetMesh Owning%20Character) (Utilities|Select :Index (Utilities|GetClassDefaults (Utilities|Struct|BreakDELETE_S_ItemData Item%20Data)) :None "shield" :OneHand "off_hand" :TwoHand "two_hand" :OffHand "shield") "SnapToTarget" "SnapToTarget" "SnapToTarget" false))))))))))

(fn DELETEDestroyEquippableActor
  (params (Slot :type DELETE%20S%20Item%20Data%20Structure))
  (bind _equipmentslot (Utilities|Struct|BreakDELETE_S_ItemData Slot))
  (bind _equipped_weapon_slot (Variables|Default|GetEquipped%20Weapon%20Slot))
  (bind _equipped_shield_slot (Variables|Default|GetEquipped%20Shield%20Slot))
  (bind _returnvalue (Utilities|Select :Index _equipmentslot :None 0 :Head 0 :Gloves 0 :Neck 0 :ChestPlate 0 :Legs 0 :Boots 0 :Weapon _equipped_weapon_slot :Shield _equipped_shield_slot :Pocket1 0 :Pocket2 0 :Pocket3 0 :Pocket4 0 :NewSlot 0))
  ;[1 0 0.02348 0.478] SERVER: Destroy Equippable Actor
  (Utilities|DELETESwitchHasOwnerAuthority
    (:Authority
      (Utilities|IsValid _returnvalue
        (:Is%20Valid
          (Actor|DestroyActor _returnvalue))))))

(fn UpdateAddedItem
  (params (Item%20Data :type DELETE%20S%20Item%20Data%20Structure))
  (Utilities|Map|Add (Variables|Default|GetEquipment%20Data) (Utilities|Struct|BreakDELETE_S_ItemData Item%20Data) Item%20Data)
  (Default|CallOnAddedtoEquipment Item%20Data)
  (Default|CallOnItemAttach Item%20Data))

(fn UpdateRemovedItem
  (params (Item%20Data :type DELETE%20S%20Item%20Data%20Structure))
  (bind _equipmentslot (Utilities|Struct|BreakDELETE_S_ItemData Item%20Data))
  (Utilities|Map|Remove (Variables|Default|GetEquipment%20Data) _equipmentslot)
  (bind _structout (Utilities|Struct|SetmembersinDELETE_S_ItemData (LocalVariables|GetL%20Empty%20Data) _equipmentslot))
  (Utilities|Map|Add (Variables|Default|GetEquipment%20Data) _equipmentslot _structout)
  (Default|CallOnRemovedfromEquipment Item%20Data)
  (Default|CallOnItemDetach Item%20Data))

(event Custom|Server%20Transfer%20Item%20from%20Inventory
  (params (Item%20Data :type DELETE%20S%20Item%20Data%20Structure) (InSlot%20Data :type DELETE%20S%20Item%20Data%20Structure) (Inventory :type DELETE%20AC%20Inventory%20Core%20Object%20Reference) (Method :type EInputMethod%20Enum :default "RightClick"))
  ;[1 0 0.04033 0.452] SERVER: Transfer Item from Inventory to Equipment
  (bind (_success _failure_message) (CallFunction|DELETETransferItemfromInventorytoEquipment Item%20Data InSlot%20Data Inventory Method))
  (CallFunction|ClientTransferItemReturnValue _success _failure_message))

(event Custom|Server%20Destroy%20Equippable%20Actor
  (params (Item%20Data :type DELETE%20S%20Item%20Data%20Structure))
  ;[1 0 0.04033 0.452] SERVER: Destroy Equippable Actor
  (CallFunction|DELETEDestroyEquippableActor Item%20Data))

(event Custom|Server%20Remove%20Item%20Quantity
  (params (Item%20Data :type DELETE%20S%20Item%20Data%20Structure) (Quantity :type Integer))
  ;[1 0 0.04033 0.452] SERVER: Remove Item Quantity
  (CallFunction|DELETERemoveItemQuantity Item%20Data Quantity))

(event Custom|Client%20Transfer%20Item%20Return%20Value
  (params (Success :type Boolean) (Failure%20Message :type Text))
  ;[0 1 0.1179 0.451] CLIENT: Transfer Item Return Value
  (if (not Success)
    (Class|DELETEBPIWidgetManager|DELETEDisplayMessageNotify(Message) (Components|GetOwner) Failure%20Message)))

(event Custom|Server%20Transfer%20Item%20from%20Equipment
  (params (Dragged%20Data :type DELETE%20S%20Item%20Data%20Structure) (InSlot%20Data :type DELETE%20S%20Item%20Data%20Structure))
  ;[1 0 0.04033 0.452] SERVER: Transfer Item from Equipment to Equipment
  (CallFunction|DELETETransferItemfromEquipmenttoEquipment Dragged%20Data InSlot%20Data))

(event Custom|Server%20Spawn%20Equippable%20Actor
  (params (Item%20Data :type DELETE%20S%20Item%20Data%20Structure) (Owning%20Character :type BP%20RPG%20Inventory%20Character%20Object%20Reference))
  ;[1 0 0.04033 0.452] SERVER: Spawn Equippable Actor and Attach to Socket
  (CallFunction|DELETESpawnandAttachEquippableActor Item%20Data Owning%20Character))

(event Custom|Client%20Update%20Added%20Item
  (params (Item%20Data :type DELETE%20S%20Item%20Data%20Structure))
  ;[0 1 0.117 0.451] CLIENT: Update Equipment Items
  (NetworkReplication|UpdateAddedItem Item%20Data))

(event Custom|Client%20Update%20Removed%20Item
  (params (Item%20Data :type DELETE%20S%20Item%20Data%20Structure))
  ;[0 1 0.117 0.451] CLIENT: Update Equipment Items
  (NetworkReplication|UpdateRemovedItem Item%20Data))

(event Custom|Initialize%20Equipment
  ;[1 1 1] Initialize Equipment Event called from Player Controller on Possess
  (CallFunction|ClientInitializeEquipment)
  (bind _asbp_rpginventory_character (Utilities|Casting|CastToBP_RPGInventoryCharacter (Pawn|GetControlledPawn (.As플레이어%20컨트롤러 (Utilities|Casting|CastToPlayerController (Components|GetOwner))))))
  (Variables|Default|SetOwning%20Character _asbp_rpginventory_character)
  ;[1 0 0.02154 0.462] Build Equipment and Initial Equipment
  (CallFunction|DELETEBuildEquipment)
  (CallFunction|DELETEBuildInitialEquipment))

(event Custom|Client%20Initialize%20Equipment
  ;[1 1 1] Build Equipment on Client Side [Multiplayer]
  (if (not (Class|KismetSystemLibrary|IsStandalone))
    (CallFunction|DELETEBuildEquipment)))