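; Player inventory component on the PlayerController, extending AC_InventoryCore to handle looting, item transfers, durability and dropping.
; Opens and closes inventory, loot bar, vendor and storage UI, switching input modes and routing interaction input.
; Server events run transfers with gold, stack and slot checks, then report to the client.
; Drops share one loot bag until inventory closes resets DroppedIndex; the item-mesh drop alternative is unfinished and unused.
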(fn OpenInventoryWidget
  (bind _returnvalue (Components|GetOwner))
  (bind _returnvalue_2 (Components|GetOwner))
  (bind _as플레이어_컨트롤러 (Utilities|Casting|CastToPlayerController _returnvalue))
  (CallFunction|DELETEPlaySoundonOpeningWidget)
  (Class|DELETEBPIWidgetManager|DELETESetActiveWidget(Message) _returnvalue_2 "Inventory")
  (Class|DELETEBPIWidgetManager|DELETESetActiveTab(Message) _returnvalue_2 "Inventory")
  (CallFunction|DELETEStartPlayerCapture2D _returnvalue)
  (bind _returnvalue_3 (UserInterface|CreateWidget (Variables|Widgets|GetInventory%20Widget%20Class) _as플레이어_컨트롤러))
  (Variables|Widgets|SetInventory%20Widget%20Ref _returnvalue_3)
  (if (not (Class|KismetSystemLibrary|HasMultipleLocalPlayers))
    (UserInterface|Viewport|AddtoViewport (Variables|Widgets|GetInventory%20Widget%20Ref) 1)
    (else
      (UserInterface|Viewport|AddtoPlayerScreen (Variables|Widgets|GetInventory%20Widget%20Ref) 1)))
  (Input|SetInputModeGameandUI _as플레이어_컨트롤러 (Variables|Widgets|GetInventory%20Widget%20Ref) "DoNotLock" true false)
  (Variables|/Script/Engine.PlayerController|SetbShowMouseCursor _as플레이어_컨트롤러 true)
  ;[0 1 0.8125] Ignore Move & Look Inputs
  (Input|SetIgnoreMoveInput _as플레이어_컨트롤러 true)
  (Input|SetIgnoreLookInput _as플레이어_컨트롤러 true))

(fn CloseInventoryWidget
  (bind _returnvalue (Components|GetOwner))
  (bind _returnvalue_2 (Components|GetOwner))
  (bind _inventory_widget_ref (Variables|Widgets|GetInventory%20Widget%20Ref))
  (bind _as플레이어_컨트롤러 (Utilities|Casting|CastToPlayerController _returnvalue_2))
  (Class|DELETEBPIWidgetManager|DELETESetActiveWidget(Message) _returnvalue "None")
  (Class|DELETEBPIWidgetManager|DELETESetActiveTab(Message) _returnvalue "None")
  (CallFunction|DELETEStopPlayerCapture2D _returnvalue_2)
  (Utilities|IsValid _inventory_widget_ref
    (:Is%20Valid
      (Widget|RemovefromParent _inventory_widget_ref))
    (:Is%20Not%20Valid
      _))
  (Input|SetInputModeGameOnly _as플레이어_컨트롤러 false)
  (Variables|/Script/Engine.PlayerController|SetbShowMouseCursor _as플레이어_컨트롤러 false)
  (Class|Controller|ResetIgnoreInputFlags _as플레이어_컨트롤러)
  ;[1 0.8218 0 0.206] Reset Dropped Index
  (CallFunction|ServerChangeDroppedIndex))

(fn OpenLootBarWidget
  (bind _returnvalue (Components|GetOwner))
  (bind _as플레이어_컨트롤러 (Utilities|Casting|CastToPlayerController _returnvalue))
  (CallFunction|DELETEPlaySoundonOpeningWidget)
  (Variables|Widgets|SetIs%20LootBar%20Open? true)
  (Variables|Widgets|SetIs%20Interactable%20Actor%20Widget%20Open true)
  (Default|ShowLootBar (.AsRPGInventory%20HUD (Utilities|Casting|CastToRPGInventory_HUD (HUD|GetHUD _as플레이어_컨트롤러))))
  (Input|SetInputModeGameandUI _as플레이어_컨트롤러 0 "DoNotLock" true false)
  (Variables|/Script/Engine.PlayerController|SetbShowMouseCursor _as플레이어_컨트롤러 true)
  ;[0.7812 1 0] Ignore Move & Look Inputs
  (Input|SetIgnoreMoveInput _as플레이어_컨트롤러 true)
  (Input|SetIgnoreLookInput _as플레이어_컨트롤러 true))

(fn CloseLootBarWidget
  (bind _returnvalue (Components|GetOwner))
  (bind _as플레이어_컨트롤러 (Utilities|Casting|CastToPlayerController _returnvalue))
  (Variables|Widgets|SetIs%20Interactable%20Actor%20Widget%20Open false)
  (Variables|Widgets|SetIs%20LootBar%20Open? false)
  (Default|HideLootBar (.AsRPGInventory%20HUD (Utilities|Casting|CastToRPGInventory_HUD (HUD|GetHUD _as플레이어_컨트롤러))))
  (Input|SetInputModeGameOnly _as플레이어_컨트롤러 false)
  (Variables|/Script/Engine.PlayerController|SetbShowMouseCursor _as플레이어_컨트롤러 false)
  (Class|Controller|ResetIgnoreInputFlags _as플레이어_컨트롤러)
  (Class|WidgetBlueprintLibrary|SetFocustoGameViewport))

(fn OpenVendorWidget
  (bind _returnvalue (Components|GetOwner))
  (bind _returnvalue_2 (Components|GetOwner))
  (bind _as플레이어_컨트롤러 (Utilities|Casting|CastToPlayerController _returnvalue_2))
  (CallFunction|DELETEPlaySoundonOpeningWidget)
  (Variables|Widgets|SetIs%20Interactable%20Actor%20Widget%20Open true)
  (Class|DELETEBPIWidgetManager|DELETESetActiveWidget(Message) _returnvalue "Vendor")
  (Class|DELETEBPIWidgetManager|DELETESetActiveTab(Message) _returnvalue "Vendor")
  (CallFunction|DELETEStartPlayerCapture2D _returnvalue_2)
  (bind _returnvalue_3 (UserInterface|CreateWidget (Variables|Widgets|GetVendor%20Widget%20Class) _as플레이어_컨트롤러))
  (Variables|Widgets|SetVendor%20Widget%20Ref _returnvalue_3)
  (if (not (Class|KismetSystemLibrary|HasMultipleLocalPlayers))
    (UserInterface|Viewport|AddtoViewport (Variables|Widgets|GetVendor%20Widget%20Ref) 1)
    (else
      (UserInterface|Viewport|AddtoPlayerScreen (Variables|Widgets|GetVendor%20Widget%20Ref) 1)))
  (Input|SetInputModeGameandUI _as플레이어_컨트롤러 (Variables|Widgets|GetVendor%20Widget%20Ref) "DoNotLock" true false)
  (Variables|/Script/Engine.PlayerController|SetbShowMouseCursor _as플레이어_컨트롤러 true)
  ;[1 1 1] Ignore Move & Look Inputs
  (Input|SetIgnoreMoveInput _as플레이어_컨트롤러 true)
  (Input|SetIgnoreLookInput _as플레이어_컨트롤러 true))

(fn CloseVendorWidget
  (bind _returnvalue (Components|GetOwner))
  (bind _returnvalue_2 (Components|GetOwner))
  (bind _vendor_widget_ref (Variables|Widgets|GetVendor%20Widget%20Ref))
  (bind _as플레이어_컨트롤러 (Utilities|Casting|CastToPlayerController _returnvalue_2))
  (Variables|Widgets|SetIs%20Interactable%20Actor%20Widget%20Open false)
  (Class|DELETEBPIWidgetManager|DELETESetActiveWidget(Message) _returnvalue "None")
  (Class|DELETEBPIWidgetManager|DELETESetActiveTab(Message) _returnvalue "None")
  (CallFunction|DELETEStopPlayerCapture2D _returnvalue_2)
  (Utilities|IsValid _vendor_widget_ref
    (:Is%20Valid
      (Widget|RemovefromParent _vendor_widget_ref))
    (:Is%20Not%20Valid
      _))
  (Input|SetInputModeGameOnly _as플레이어_컨트롤러 false)
  (Variables|/Script/Engine.PlayerController|SetbShowMouseCursor _as플레이어_컨트롤러 false)
  (Class|Controller|ResetIgnoreInputFlags _as플레이어_컨트롤러))

(fn OpenStorageWidget
  (bind _returnvalue (Components|GetOwner))
  (bind _returnvalue_2 (Components|GetOwner))
  (bind _as플레이어_컨트롤러 (Utilities|Casting|CastToPlayerController _returnvalue_2))
  (CallFunction|DELETEPlaySoundonOpeningWidget)
  (Variables|Widgets|SetIs%20Interactable%20Actor%20Widget%20Open true)
  (Class|DELETEBPIWidgetManager|DELETESetActiveWidget(Message) _returnvalue "Storage")
  (Class|DELETEBPIWidgetManager|DELETESetActiveTab(Message) _returnvalue "Storage")
  (CallFunction|DELETEStartPlayerCapture2D _returnvalue_2)
  (bind _returnvalue_3 (UserInterface|CreateWidget (Variables|Widgets|GetStorage%20Widget%20Class) _as플레이어_컨트롤러))
  (Variables|Widgets|SetStorage%20Widget%20Ref _returnvalue_3)
  (if (not (Class|KismetSystemLibrary|HasMultipleLocalPlayers))
    (UserInterface|Viewport|AddtoViewport (Variables|Widgets|GetStorage%20Widget%20Ref) 1)
    (else
      (UserInterface|Viewport|AddtoPlayerScreen (Variables|Widgets|GetStorage%20Widget%20Ref) 1)))
  (Input|SetInputModeGameandUI _as플레이어_컨트롤러 (Variables|Widgets|GetStorage%20Widget%20Ref) "DoNotLock" true false)
  (Variables|/Script/Engine.PlayerController|SetbShowMouseCursor _as플레이어_컨트롤러 true)
  ;[1 1 1] Ignore Move & Look Inputs
  (Input|SetIgnoreMoveInput _as플레이어_컨트롤러 true)
  (Input|SetIgnoreLookInput _as플레이어_컨트롤러 true))

(fn CloseStorageWidget
  (bind _returnvalue (Components|GetOwner))
  (bind _returnvalue_2 (Components|GetOwner))
  (bind _storage_widget_ref (Variables|Widgets|GetStorage%20Widget%20Ref))
  (bind _as플레이어_컨트롤러 (Utilities|Casting|CastToPlayerController _returnvalue))
  (Variables|Widgets|SetIs%20Interactable%20Actor%20Widget%20Open false)
  (Class|DELETEBPIWidgetManager|DELETESetActiveWidget(Message) _returnvalue_2 "None")
  (Class|DELETEBPIWidgetManager|DELETESetActiveTab(Message) _returnvalue_2 "None")
  (CallFunction|DELETEStopPlayerCapture2D _returnvalue)
  (Utilities|IsValid _storage_widget_ref
    (:Is%20Valid
      (Widget|RemovefromParent _storage_widget_ref))
    (:Is%20Not%20Valid
      _))
  (Input|SetInputModeGameOnly _as플레이어_컨트롤러 false)
  (Variables|/Script/Engine.PlayerController|SetbShowMouseCursor _as플레이어_컨트롤러 false)
  (Class|Controller|ResetIgnoreInputFlags _as플레이어_컨트롤러))

(fn TakeItem
  (params (Item%20Data :type DELETE%20S%20Item%20Data%20Structure) (Sender :type DELETE%20AC%20Inventory%20Core%20Object%20Reference))
  (Utilities|DELETEIsItemClassValid? Item%20Data
    (:Valid
      (bind _output_get (LocalVariables|SetL%20Item Item%20Data))
      (bind (_success _failure_message) (CallFunction|DELETETransferItemfromInventory :Item%20Data _output_get :Sender Sender))
      (CallFunction|ClientTakeItemReturnValue _success _failure_message (not (Utilities|Array|IsValidIndex (.Inventory (Default|DELETEGetInventoryandSize Sender "P1")))))
      (if _success
        (CallFunction|ClientItemLooted (LocalVariables|GetL%20Item))))))

(fn TakeAllItems
  (params (Sender :type DELETE%20AC%20Inventory%20Core%20Object%20Reference))
  (bind _output_get (LocalVariables|SetL%20Items (.Inventory (Default|DELETEGetInventoryandSize Sender "P1"))))
  (bind _array_element (Utilities|Array|ForEachLoopwithBreak _output_get :!label _label)
    (:LoopBody
      (Utilities|DELETEIsItemClassValid? _array_element
        (:Valid
          (bind _output_get_2 (LocalVariables|SetL%20Item _array_element))
          (bind (_success _failure_message) (CallFunction|DELETETransferItemfromInventory :Item%20Data _output_get_2 :Sender Sender))
          (if _success
            (CallFunction|ClientItemLooted (LocalVariables|GetL%20Item))
            (else
              (LocalVariables|SetL%20FailureMessage _failure_message)
              (LocalVariables|SetL%20ReturnValue false)
              (goto _label Break))))))
    (:Completed
      (CallFunction|ClientTakeItemReturnValue (LocalVariables|GetL%20ReturnValue) (LocalVariables|GetL%20FailureMessage) (not (Utilities|Array|IsValidIndex (.Inventory (Default|DELETEGetInventoryandSize Sender "P1"))))))))

(fn IncreaseItemDurability
  (params (Item%20Data :type DELETE%20S%20Item%20Data%20Structure%20%28by%20ref%29) (Amount :type Integer))
  (bind (_class _durability) (Utilities|Struct|BreakDELETE_S_ItemData Item%20Data))
  (bind _returnvalue (Components|GetOwner))
  (bind _returnvalue_2 (Actor|GetComponentbyClass _returnvalue "/Game/InventorySystem/Blueprints/Components/DELETE_AC_PlayerEquipment.DELETE_AC_PlayerEquipment_C"))
  (if (Utilities|GetClassDefaults _class)
    (bind _structout (Utilities|Struct|SetmembersinDELETE_S_ItemData Item%20Data (Math|Integer|Clamp(Integer) (+ _durability Amount) 0 100)))
    (bind _output_get (LocalVariables|SetL%20Item%20Data _structout))
    (if (Utilities|Struct|BreakDELETE_S_ItemData _output_get)
      ;[1 0 0 0.504] Override Changes in Player Equipment
      (Utilities|IsValid _returnvalue_2
        (:Is%20Valid
          (Default|DELETERemoveItemfromEquipmentArray _returnvalue_2 (LocalVariables|GetL%20Item%20Data))
          (Default|DELETEAddItemtoEquipmentArray _returnvalue_2 (LocalVariables|GetL%20Item%20Data) (Utilities|Struct|BreakDELETE_S_ItemData (LocalVariables|GetL%20Item%20Data)))))
      (else
        ;[0 1 0.2146 0.467] Override Changes in Player Inventory
        (CallFunction|DELETEAddItemtoInventoryArray (LocalVariables|GetL%20Item%20Data) (.Index (Utilities|Struct|BreakDELETE_S_ItemData (LocalVariables|GetL%20Item%20Data))))))))

(fn DecreaseItemDurability
  (params (Item%20Data :type DELETE%20S%20Item%20Data%20Structure%20%28by%20ref%29) (Amount :type Integer))
  (bind (_class _durability) (Utilities|Struct|BreakDELETE_S_ItemData Item%20Data))
  (bind _returnvalue (Components|GetOwner))
  (bind _returnvalue_2 (Actor|GetComponentbyClass _returnvalue "/Game/InventorySystem/Blueprints/Components/DELETE_AC_PlayerEquipment.DELETE_AC_PlayerEquipment_C"))
  (if (Utilities|GetClassDefaults _class)
    (bind _structout (Utilities|Struct|SetmembersinDELETE_S_ItemData Item%20Data (Math|Integer|Clamp(Integer) (- _durability Amount) 0 100)))
    (bind _output_get (LocalVariables|SetL%20Item%20Data _structout))
    (if (Utilities|Struct|BreakDELETE_S_ItemData _output_get)
      ;[1 0 0 0.504] Override Changes in Player Equipment
      (Utilities|IsValid _returnvalue_2
        (:Is%20Valid
          (Default|DELETERemoveItemfromEquipmentArray _returnvalue_2 (LocalVariables|GetL%20Item%20Data))
          (Default|DELETEAddItemtoEquipmentArray _returnvalue_2 (LocalVariables|GetL%20Item%20Data) (Utilities|Struct|BreakDELETE_S_ItemData (LocalVariables|GetL%20Item%20Data)))))
      (else
        ;[0 1 0.2146 0.467] Override Changes in Player Inventory
        (CallFunction|DELETEAddItemtoInventoryArray (LocalVariables|GetL%20Item%20Data) (.Index (Utilities|Struct|BreakDELETE_S_ItemData (LocalVariables|GetL%20Item%20Data))))))))

(fn DropItemontheGround
  (params (Item%20Data :type DELETE%20S%20Item%20Data%20Structure) (Initiator :type EItemDestination%20Enum :default "None"))
  (switch Utilities|FlowControl|Switch|SwitchonEItemDestination Initiator
    (:None
      (CallFunction|DELETERemoveItemfromInventoryArray Item%20Data :!label _label))
    (:InventorySlot
      (goto _label))
    (:EquipmentSlot
      (bind _output_get (LocalVariables|SetL%20Equipment (Actor|GetComponentbyClass (Components|GetOwner) "/Game/InventorySystem/Blueprints/Components/DELETE_AC_PlayerEquipment.DELETE_AC_PlayerEquipment_C")))
      (Default|DELETERemoveItemfromEquipmentArray _output_get Item%20Data)
      (Default|DELETEDetachItemfromEquipment (LocalVariables|GetL%20Equipment) Item%20Data)))
  (CallFunction|DELETERemoveWeightfromInventory (Utilities|DELETECalculateStackedItemWeight Item%20Data))
  (CallFunction|ServerSpawnLootBag Item%20Data))

(fn SpawnLootBagNearthePlayer
  (params (Item%20Data :type DELETE%20S%20Item%20Data%20Structure))
  (bind _as컨트롤러 (Utilities|Casting|CastToController (Components|GetOwner)))
  (if (>= (Variables|Default|GetDroppedIndex) 1)
    _
    (elif (.Return%20Value (CallFunction|IsCollidingwithLootBag (- (+ (Transformation|GetActorLocation (Pawn|GetControlledPawn _as컨트롤러)) (* (Transformation|GetActorForwardVector (Pawn|GetControlledPawn _as컨트롤러)) 5e+01)) "0, 0,50.000000") (- (- (+ (Transformation|GetActorLocation (Pawn|GetControlledPawn _as컨트롤러)) (* (Transformation|GetActorForwardVector (Pawn|GetControlledPawn _as컨트롤러)) 5e+01)) "0, 0,50.000000") "0, 0,100.000000")))
      (Variables|Default|SetLootBag%20Ref (.Dropped%20Bag (CallFunction|IsCollidingwithLootBag (- (+ (Transformation|GetActorLocation (Pawn|GetControlledPawn _as컨트롤러)) (* (Transformation|GetActorForwardVector (Pawn|GetControlledPawn _as컨트롤러)) 5e+01)) "0, 0,50.000000") (- (- (+ (Transformation|GetActorLocation (Pawn|GetControlledPawn _as컨트롤러)) (* (Transformation|GetActorForwardVector (Pawn|GetControlledPawn _as컨트롤러)) 5e+01)) "0, 0,50.000000") "0, 0,100.000000"))))
      (else
        (bind _returnvalue (Game|SpawnActorfromClass "/Game/InventorySystem/Classes/Interactable/BP_LootBag.BP_LootBag_C" (Math|Transform|MakeTransform (- (+ (Transformation|GetActorLocation (Pawn|GetControlledPawn _as컨트롤러)) (* (Transformation|GetActorForwardVector (Pawn|GetControlledPawn _as컨트롤러)) 5e+01)) "0, 0,50.000000")) "Undefined" "OverrideRootScale" (Components|GetOwner) 0))
        (Variables|Default|SetLootBag%20Ref _returnvalue))))
  (Variables|Default|SetDroppedIndex (+ (Variables|Default|GetDroppedIndex) 1))
  (Utilities|IsValid (Actor|GetComponentbyClass (Variables|Default|GetLootBag%20Ref) "/Game/InventorySystem/Blueprints/Components/DELETE_AC_InventoryCore.DELETE_AC_InventoryCore_C")
    (:Is%20Valid
      (bind _output_get (LocalVariables|SetL%20Receiver%20Inventory (Actor|GetComponentbyClass (Variables|Default|GetLootBag%20Ref) "/Game/InventorySystem/Blueprints/Components/DELETE_AC_InventoryCore.DELETE_AC_InventoryCore_C")))
      (bind _slot_index (Utilities|DELETEHasPartialStack? (.Inventory (Default|DELETEGetInventoryandSize _output_get (Utilities|DELETEGetInventoryPanelfromItem Item%20Data))) Item%20Data)
        (:True
          (Default|DELETEAddtoStackinInventory (LocalVariables|GetL%20Receiver%20Inventory) Item%20Data _slot_index))
        (:False
          (Default|DELETEAddItemtoInventoryArray (LocalVariables|GetL%20Receiver%20Inventory) Item%20Data -1))))))

(fn SpawnItemMeshNearthePlayer
  (params (Item%20Data :type DELETE%20S%20Item%20Data%20Structure))
  (bind _as컨트롤러 (Utilities|Casting|CastToController (Components|GetOwner)))
  (bind _output_get (LocalVariables|SetL%20Base%20Item%20Ref 0))
  (Default|MulticastSetPhysicsSimulation _output_get)
  (Variables|Default|SetDroppedIndex (+ (Variables|Default|GetDroppedIndex) 1))
  (Utilities|IsValid (Actor|GetComponentbyClass (LocalVariables|GetL%20Base%20Item%20Ref) "/Game/InventorySystem/Blueprints/Components/DELETE_AC_InventoryCore.DELETE_AC_InventoryCore_C")
    (:Is%20Valid
      (bind _output_get_2 (LocalVariables|SetL%20Receiver%20Inventory (Actor|GetComponentbyClass (LocalVariables|GetL%20Base%20Item%20Ref) "/Game/InventorySystem/Blueprints/Components/DELETE_AC_InventoryCore.DELETE_AC_InventoryCore_C")))
      (bind _slot_index (Utilities|DELETEHasPartialStack? (.Inventory (Default|DELETEGetInventoryandSize _output_get_2 (Utilities|DELETEGetInventoryPanelfromItem Item%20Data))) Item%20Data)
        (:True
          (Default|DELETEAddtoStackinInventory (LocalVariables|GetL%20Receiver%20Inventory) Item%20Data _slot_index))
        (:False
          (Default|DELETEAddItemtoInventoryArray (LocalVariables|GetL%20Receiver%20Inventory) Item%20Data -1))))))

(fn IsCollidingwithLootBag
  (params (Start :type Vector) (End :type Vector))
  (bind (_outhit _returnvalue) (Collision|LineTraceByChannel Start End "TraceTypeQuery1" false 0 "None"))
  (if _returnvalue
    (bind _asbp_loot_bag (Utilities|Casting|CastToBP_LootBag (.HitActor (Collision|BreakHitResult _outhit)))
      (:then
        (return true _asbp_loot_bag))
      (:CastFailed
        (return false 0)))
    (else
      (return false 0))))

(fn DELETETransferItemfromInventory
  (params (Item%20Data :type DELETE%20S%20Item%20Data%20Structure%20%28by%20ref%29) (In%20Slot%20Data :type DELETE%20S%20Item%20Data%20Structure) (Method :type EInputMethod%20Enum :default "RightClick") (Sender :type DELETE%20AC%20Inventory%20Core%20Object%20Reference))
  (bind _returnvalue (Components|GetOwner))
  (bind _returnvalue_2 (Actor|GetComponentbyClass _returnvalue "/Game/InventorySystem/Blueprints/Components/DELETE_AC_PlayerEquipment.DELETE_AC_PlayerEquipment_C"))
  (bind (_slot_found _slot_index) (CallFunction|DELETEGetEmptyInventorySlot Item%20Data))
  (bind _output_get (LocalVariables|SetL%20Item%20Data Item%20Data))
  (Utilities|DELETEIsItemClassValid? _output_get
    (:Valid
      (Utilities|IsValid Sender
        (:Is%20Valid
          ;[1 0 0.01726 0.352] Check #1 If Item is a Currency - Add Gold to Owner and Remove Item from Sender Inventory [Normally should only work when Transferring to the Player Inventory]
          (if (not (Utilities|DELETEIsItemACurrency? (LocalVariables|GetL%20Item%20Data)))
            ;[1 0 0.01726 0.352] Check #2 Has owner enough Gold [Bypass if Sender or Receiver has 'Check Owner Gold' set to False]
            (if (Variables|/Game/InventorySystem/Blueprints/Components/DELETE_AC_InventoryCore.DELETE_AC_InventoryCore_C|GetCheck%20Owner%20Gold Sender)
              (if (CallFunction|DELETEHasEnoughGold? Item%20Data)
                _
                (else
                  (return false (Variables|Default|GetMessageNotEnoughGold)))))
            ;[1 0.6397 0 0.373] Additional Check # Has Partial Stack in Equipment? If so Add to Stack
            (Utilities|IsValid _returnvalue_2
              (:Is%20Valid
                (bind _success (Default|DELETETrytoAddtoPartialStack _returnvalue_2 Item%20Data))
                (if _success
                  _
                  (else
                    ;[1 0.6397 0 0.373] Check #3 Has Partial Stack? If so Add to Stack in Inventory
                    (bind _slot_index_2 (Utilities|DELETEHasPartialStack? (.Inventory (CallFunction|DELETEGetInventoryandSize (Utilities|DELETEGetInventoryPanelfromItem Item%20Data))) Item%20Data :!label _label)
                      (:True
                        (CallFunction|DELETEAddtoStackinInventory Item%20Data _slot_index_2))
                      (:False
                        ;[0.1981 0 1 0.535] Switch on Input Method
                        (switch Utilities|FlowControl|Switch|SwitchonEInputMethod Method
                          (:RightClick
                            ;[0 1 0.007759 0.54] Check #4 Has Empty Slot in Inventory? If so Add Item to that Slot Index
                            (if _slot_found
                              (CallFunction|DELETEAddItemtoInventoryArray Item%20Data _slot_index)
                              (else
                                (return false (Variables|Default|GetMessageInventoryFull)))))
                          (:DragAndDrop
                            ;[0 1 0.007759 0.54] Add to specified Slot in Inventory
                            (CallFunction|DELETEAddItemtoInventoryArray Item%20Data (Utilities|Struct|BreakDELETE_S_ItemData In%20Slot%20Data)))))))))
              (:Is%20Not%20Valid
                (goto _label)))
            ;[0 1 0.007499 0.5412] Add Item Weight to Receiver Inventory
            (CallFunction|DELETEAddWeighttoInventory (Utilities|DELETECalculateStackedItemWeight Item%20Data))
            ;[1 0 0.01681 0.3529] Remove Gold / Add Gold to Owner [Only if both Sender and Receiver has 'Check Owner Gold' set to True]
            (if (and (Variables|/Game/InventorySystem/Blueprints/Components/DELETE_AC_InventoryCore.DELETE_AC_InventoryCore_C|GetCheck%20Owner%20Gold Sender) (Variables|Default|GetCheck%20Owner%20Gold))
              (CallFunction|DELETERemoveGoldfromOwner (Utilities|DELETECalculateStackedItemValue (LocalVariables|GetL%20Item%20Data)))
              (Default|DELETEAddGoldtoOwner Sender (Utilities|DELETECalculateStackedItemValue (LocalVariables|GetL%20Item%20Data))))
            ;[0 1 0.007499 0.5412] Remove Item and Item Weight from Sender Inventory
            (Default|DELETERemoveItemfromInventoryArray Sender (LocalVariables|GetL%20Item%20Data))
            (Utilities|IsValid Sender ; Does Sender Owner still exist?
              (:Is%20Valid
                (Default|DELETERemoveWeightfromInventory Sender (Utilities|DELETECalculateStackedItemWeight (LocalVariables|GetL%20Item%20Data))))
              (:Is%20Not%20Valid
                _))
            (return true "")
            (else
              (CallFunction|DELETEAddGoldtoOwner (Utilities|DELETECalculateStackedItemValue (LocalVariables|GetL%20Item%20Data)))
              (Default|DELETERemoveItemfromInventoryArray Sender (LocalVariables|GetL%20Item%20Data))
              (return true ""))))
        (:Is%20Not%20Valid
          _)))
    (:Not%20Valid
      _))
  (return false ""))

(fn DELETESplitItemsinInventory
  (params (Sender :type DELETE%20AC%20Inventory%20Core%20Object%20Reference) (Item%20Data :type DELETE%20S%20Item%20Data%20Structure) (In%20Slot%20Data :type DELETE%20S%20Item%20Data%20Structure) (Stackable%20Left :type DELETE%20S%20Item%20Data%20Structure) (Input%20Method :type EInputMethod%20Enum :default "RightClick") (Initiator :type EItemDestination%20Enum :default "None") (Destination :type EItemDestination%20Enum :default "None")))

(fn DELETEConfirmationPopupAccepted
  (params (Sender :type DELETE%20AC%20Inventory%20Core%20Object%20Reference) (Item%20Data :type DELETE%20S%20Item%20Data%20Structure) (In%20Slot%20Data :type DELETE%20S%20Item%20Data%20Structure) (Input%20Method :type EInputMethod%20Enum :default "RightClick") (Initiator :type EItemDestination%20Enum :default "None") (Destination :type EItemDestination%20Enum :default "None"))
  (Utilities|DELETEIsStackableandHaveStacks? Item%20Data 1))

(event Custom|Bind%20Events
  ;[0 0.1927 1 0.509] Interaction Binding
  (bind _ac_interaction (CallFunction|DELETEGetACInteraction (Components|GetOwner)))
  (EventDispatchers|BindEventtoOnNewInteractableAssigned _ac_interaction (EventDispatchers|CreateEvent :!event Custom|Set%20New%20Interactable))
  (EventDispatchers|BindEventtoOnRemovedCurrentInteractable _ac_interaction (EventDispatchers|CreateEvent :!event Custom|Remove%20Current%20Interactable)))

(event Custom|Remove%20Current%20Interactable
  ;[1 0.05204 0 0.379] Remove Current Interactable
  (Variables|Default|SetCurrent%20Interactable 0))

(event Custom|Set%20New%20Interactable
  (params (Current%20Interactable :type DELETE%20AC%20Interactable%20Object%20Reference))
  ;[0 1 0.1257 0.379] Set New Interactable
  (Variables|Default|SetCurrent%20Interactable Current%20Interactable))

(event EventDELETEInitializeInventory
  ;[1 0.07031 0] Event Initialize Inventory [Called on Possess]
  (|CallParentFunction))

(event EventBeginPlay
  ;[1 0.7266 0] Instead of Event Begin Player use Event Initialize Inventory [Called from owner]
)

(event EventDELETEClientInitializeInventory
  ;[0.6641 0 1] Event Client Initialize Inventory called on Initialize Inventory - Inside AC_InventoryCore
  (|CallParentFunction) ; Run Build Inventory Logic on Client Side
  ;[1 0.0258 0 0.311] Bind Event Dispatchers
  (CallFunction|BindEvents))

(event Custom|Input%20TakeAll
  ;[1 0.01637 0 0.525] Input - Take All
  (if (Variables|Widgets|GetIs%20LootBar%20Open?)
    (Default|CallOnTakeAllItems)))

(event Custom|Input%20Interaction
  ;[1 0.01637 0 0.525] Input - Interaction
  (Utilities|FlowControl|Delay 0.0)
  (if (Variables|Widgets|GetIs%20LootBar%20Open?)
    (Default|CallOnTakeItem) ; Function Called inside WB_LootBar
    (elif (not (Variables|Widgets|GetIs%20Interactable%20Actor%20Widget%20Open))
      (bind _current_interactable (Variables|Default|GetCurrent%20Interactable)
        (:then
          (Class|DELETEBPIObjectInteraction|InitializeInteractionwithObject(Message) (Components|GetOwner) _current_interactable))
        (:else)))))

(event Custom|Input%20Close%20Widget
  (bind _returnvalue (Components|GetOwner))
  ;[1 0.01637 0 0.525] Input - Close Widget
  (if (Variables|Widgets|GetIs%20Interactable%20Actor%20Widget%20Open)
    (Class|DELETEBPIObjectInteraction|EndInteractionwithObject(Message) _returnvalue (Variables|Default|GetCurrent%20Interactable))
    (else
      (Class|DELETEBPIWidgetManager|DELETECloseActiveWidget(Message) _returnvalue))))

(event Custom|Input%20Inventory
  ;[1 0.01637 0 0.525] Input - Inventory
  (if (Variables|Widgets|GetIs%20LootBar%20Open?)
    (Class|DELETEBPIObjectInteraction|EndInteractionwithObject(Message) (Components|GetOwner) (Variables|Default|GetCurrent%20Interactable)))
  (bind _widget (Class|DELETEBPIWidgetManager|DELETEGetActiveWidget(Message) (Components|GetOwner)))
  (if (Utilities|Enum|Equal(Enum) _widget "Inventory")
    (Widgets|CloseInventoryWidget)
    (else
      (if (Variables|Widgets|GetIs%20Interactable%20Actor%20Widget%20Open)
        (Class|DELETEBPIObjectInteraction|EndInteractionwithObject(Message) (Components|GetOwner) (Variables|Default|GetCurrent%20Interactable)))
      (Class|DELETEBPIWidgetManager|DELETESwitchWidgetto(Message) (Components|GetOwner) "Inventory"))))

(event Custom|Server%20Change%20Dropped%20Index
  (params (DroppedIndex :type Integer))
  ;[1 0.00746 0 0.525 24] SERVER EVENTS
  (Variables|Default|SetDroppedIndex DroppedIndex))

(event Custom|Client%20Take%20Item%20Return%20Value
  (params (Success :type Boolean) (Failure%20Message :type Text) (Remove%20Interaction :type Boolean))
  ;[0 1 0.04606 0.525 24] CLIENT EVENTS
  (|TakeItemReturnValue Success Failure%20Message Remove%20Interaction))

(event Custom|Server%20Take%20All%20Items
  (params (Sender :type DELETE%20AC%20Inventory%20Core%20Object%20Reference))
  ;[1 0.00746 0 0.525 24] SERVER EVENTS
  (CallFunction|TakeAllItems Sender))

(event Custom|Server%20Drop%20Item%20on%20the%20Ground
  (params (Item%20Data :type DELETE%20S%20Item%20Data%20Structure) (Initiator :type EItemDestination%20Enum :default "None"))
  ;[1 0.00746 0 0.525 24] SERVER EVENTS
  (CallFunction|DropItemontheGround Item%20Data Initiator))

(event Custom|Server%20Spawn%20LootBag
  (params (Item%20Data :type DELETE%20S%20Item%20Data%20Structure))
  ;[1 0.00746 0 0.525 24] SERVER EVENTS
  (CallFunction|SpawnLootBagNearthePlayer Item%20Data))

(event Custom|Server%20Take%20Item
  (params (Item%20Data :type DELETE%20S%20Item%20Data%20Structure) (Sender :type DELETE%20AC%20Inventory%20Core%20Object%20Reference))
  ;[1 0.00746 0 0.525 24] SERVER EVENTS
  (CallFunction|TakeItem Item%20Data Sender))

(event Custom|Client%20Item%20Looted
  (params (Looted%20Item :type DELETE%20S%20Item%20Data%20Structure))
  ;[0 1 0.04606 0.525 24] CLIENT EVENTS
  (Default|CallOnItemLooted Looted%20Item))

(event Custom|Server%20Spawn%20Interactable
  (params (Item%20Data :type DELETE%20S%20Item%20Data%20Structure))
  ;[1 0.00746 0 0.525 24] SERVER EVENTS
  (CallFunction|SpawnItemMeshNearthePlayer Item%20Data))