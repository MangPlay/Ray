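; Actor component, prefixed DELETE, that makes its owner interactable, with outline highlighting and a prompt widget.
; Pre-interaction handles single, hold or mash input, animating the widget fill before asking the interactor to start interacting.
; Owners receive lifecycle messages for initialization, interaction, end, removal and game load, with response type governing removal and re-initialization.
; Associated actors can act as triggers, optionally firing the main interactable only when their values match targets.
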(fn ToggleIsInteractable
  (params (Condition :type Boolean))
  (if (Math|Boolean|NotEqual(Boolean) Condition (Variables|Main|GetIsInteractable))
    (Variables|Main|SetIsInteractable Condition)))

(fn FillInteractionWidgetBorder
  (params (Value :type Float%20%28double-precision%29))
  (Utilities|IsValid (Variables|Interaction|GetInteraction%20Widget%20Ref)
    (:Is%20Valid
      (Default|EventBorderFill (Variables|Interaction|GetInteraction%20Widget%20Ref) (Math|Float|MapRangeClamped Value 0.0 (Variables|Interaction|GetMax%20Key%20Time%20Down) 0.0 1.0)))))

(fn ToggleInteractionWidget
  (params (Condition :type Boolean))
  (bind _interaction_widget_ref (Variables|Interaction|GetInteraction%20Widget%20Ref))
  (if (Variables|Main|GetIsInteractable)
    (Utilities|IsValid _interaction_widget_ref
      (:Is%20Valid
        (Widget|SetVisibility _interaction_widget_ref (select Condition "Visible" "Hidden"))
        (Default|SetFillDecimalValue _interaction_widget_ref 0.05)))))

(fn RemoveInteractionbyResponse
  (switch Utilities|FlowControl|Switch|SwitchonEInteractionResponse (Variables|Interaction|GetInteractable%20Response)
    (:OnlyOnce
      _)
    (:Temporary
      _))
  (CallFunction|EventRemoveInteraction))

(fn ChangeInteractableValue
  (params (Increment :type Boolean))
  (if Increment
    (bind _result (Math|Integer|IncrementInt (Variables|Interaction|GetInteractable%20Value))
      (:%20%20
        (if (> _result (Variables|Interaction|GetInteractable%20Limit%20Value))
          (Variables|Interaction|SetInteractable%20Value 0))))
    (else
      (bind _result_2 (Math|Integer|DecrementInt (Variables|Interaction|GetInteractable%20Value))
        (:%20%20
          (if (< _result_2 0)
            (Variables|Interaction|SetInteractable%20Value (Variables|Interaction|GetInteractable%20Limit%20Value))))))))

(fn ToggleCanbeReInitialized
  (params (Condition :type Boolean))
  (if (Math|Boolean|NotEqual(Boolean) Condition (Variables|Interaction|GetCan%20be%20ReInitialized?))
    (Variables|Interaction|SetCan%20be%20ReInitialized? Condition)))

(fn SetWidgetLocalOwner
  (params (OwningPlayer :type Player%20Controller%20Object%20Reference))
  (bind _interaction_widget (Variables|Default|GetInteraction%20Widget))
  (bind _returnvalue (UserInterface|CreateWidget "/Game/InventorySystem/UI/Misc/Interaction/WB_Interaction.WB_Interaction_C" OwningPlayer (Variables|Interaction|GetDefaultInteractionText) (Variables|Interaction|GetInput%20Type)))
  (bind _output_get (Variables|Interaction|SetInteraction%20Widget%20Ref _returnvalue))
  (UserInterface|SetWidget _interaction_widget _output_get)
  (Class|WidgetComponent|SetOwnerPlayer _interaction_widget (Class|Widget|GetOwningLocalPlayer _output_get)))

(event EventBeginPlay
  ;[1 0.01949 0 0.452] On Begin Play - Call Event Initialize and set appropriate Tags to Component Owners
  (CallFunction|EventInitialize)
  (Utilities|Array|AddUnique (Variables|/Script/Engine.Actor|GetTags (Components|GetOwner)) (Variables|Interaction|GetInteractable%20Tag))
  (if (Variables|Interaction|GetDestroy%20after%20Pickup?)
    (Utilities|Array|AddUnique (Variables|/Script/Engine.Actor|GetTags (Components|GetOwner)) (Variables|Interaction|GetDestroyable%20Tag))))

(event Custom|Debug%20Toggle%20Owner%20Name
  (params (IsDebugging :type Boolean) (Duration :type Float%20%28double-precision%29))
  (if IsDebugging
    (Rendering|Debug|DrawDebugString (Transformation|GetWorldLocation (Variables|Default|GetInteraction%20Widget)) (Utilities|GetDisplayName (Components|GetOwner)) 0 "(R=1.000000,G=0.000000,B=0.024906,A=1.000000)" Duration)
    (else
      (Class|KismetSystemLibrary|FlushDebugStrings))))

(event Custom|Debug%20Toggle%20Interactable%20Area
  (params (IsDebugging :type Boolean))
  (bind _interactable_area (Variables|Default|GetInteractable%20Area))
  (Utilities|IsValid _interactable_area
    (:Is%20Valid
      (Development|SetHiddeninGame _interactable_area (select IsDebugging false true) false))))

(event Custom|Debug%20Toggle%20Object%20Highlight
  (params (IsDebugging :type Boolean))
  (Rendering|SetRenderCustomDepth (Variables|Interaction|GetObjects%20to%20Highlight) IsDebugging))

(event Custom|Event%20Check%20for%20Interaction%20with%20Associate
  (params (Interactor :type Actor%20Object%20Reference))
  ;[0 0 0 0.426 22] [On Interaction with Associated Actor]
  ;
  ; 1. Is called from Interactable Object that is used as a Trigger for the main Interactable
  ; 2. If 'Check for Associated Actors' is marked as True:
  ;  Check if each Associated Actor has proper Interactable Value assigned
  ;  Call Event Interaction for the Main Interactable
  ;  Remove Interaction by Response for each Associated Actor
  ;;[1 0 0 0.2] 2. Check for Interaction with Associated Actors
  (Variables|Default|SetInteractor Interactor)
  (if (Variables|Interaction|GetCheck%20for%20Associated%20Actors)
    (Utilities|IsTargetInteractableValue
      (:True
        _)))
  (CallFunction|EventInteraction (Variables|Default|GetInteractor))
  (if (Variables|Interaction|GetRemove%20Associated%20Interactables%20On%20Complete)
    (bind _keys (Utilities|Map|Keys (Variables|Interaction|GetAssociated%20Interactable%20Actors) :!label _label))
    (for _array_element _keys
      (CallFunction|EventRemoveInteraction (Actor|GetComponentbyClass _array_element "DELETE_AC_Interactable_C"))
      (Variables|DELETE_AC_Interactable_C|SetInteractable%20Response (Actor|GetComponentbyClass _array_element "DELETE_AC_Interactable_C") "OnlyOnce"))
    (else
      (switch Utilities|FlowControl|Switch|SwitchonEInteractionResponse (Variables|Interaction|GetInteractable%20Response)
        (:OnlyOnce
          (goto _label))
        (:Temporary
          (bind _keys_2 (Utilities|Map|Keys (Variables|Interaction|GetAssociated%20Interactable%20Actors)))
          (for _array_element_2 _keys_2
            (CallFunction|EventRemoveInteraction (Actor|GetComponentbyClass _array_element_2 "DELETE_AC_Interactable_C"))
            (Interaction|ToggleCanbeReInitialized (Actor|GetComponentbyClass _array_element_2 "DELETE_AC_Interactable_C") false)))))))

(event Custom|Event%20Interaction
  (params (Interactor :type Actor%20Object%20Reference))
  ;[0 0 0 0.426 22] [On Interaction]
  ;
  ; Set Object as Already Interacted [Boolean]
  ; Call Event Interaction inside Interactable Object
  ; Remove Interaction if Persitent Response is not selected
  ;;[1 0 0 0.2] On Interaction
  (Variables|Default|SetInteractor Interactor)
  (Variables|Interaction|SetAlready%20Interacted true)
  (Class|DELETEBPIInteractable|Interaction(Message) (Components|GetOwner) (Variables|Default|GetInteractor))
  (Interaction|RemoveInteractionbyResponse))

(event Custom|Event%20Associated%20Actor%20Interaction
  (params (Interactor :type Actor%20Object%20Reference))
  ;[0 0 0 0.426 22] [On Interaction with Associated Actor]
  ;
  ; 1. Is called from Interactable Object that is used as a Trigger for the main Interactable
  ; 2. If 'Check for Associated Actors' is marked as True:
  ;  Check if each Associated Actor has proper Interactable Value assigned
  ;  Call Event Interaction for the Main Interactable
  ;  Remove Interaction by Response for each Associated Actor
  ;;[1 0 0 0.2] 1. Fire Event Interaction in each Associated Actor
  (Variables|Default|SetInteractor Interactor)
  (bind _keys (Utilities|Map|Keys (Variables|Interaction|GetAssociated%20Interactable%20Actors)))
  (for _array_element _keys
    (Utilities|IsValid _array_element
      (:Is%20Valid
        (Utilities|IsValid (Actor|GetComponentbyClass _array_element "DELETE_AC_Interactable_C")
          (:Is%20Valid
            (CallFunction|EventCheckforInteractionwithAssociate (Actor|GetComponentbyClass _array_element "DELETE_AC_Interactable_C") (Variables|Default|GetInteractor))))))))

(event Custom|Event%20Toggle%20Highlight
  (params (Highlight :type Boolean) (Interactor :type Actor%20Object%20Reference))
  ;[0 0 0 0.426 22] [On Approach]
  ;
  ; 1. Toggle Interaction Widget & Objects Outlines
  ;
  ; This Event is called from Interaction Component / 'Assign Interaction' or 'Remove Interaction'
  ;;[1 0 0 0.201] Toggle Highlight
  (Rendering|SetVisibility (Variables|Default|GetInteraction%20Widget) Highlight false)
  (Rendering|SetRenderCustomDepth (Variables|Interaction|GetObjects%20to%20Highlight) Highlight)
  (CallFunction|SetWidgetLocalOwner (.As플레이어%20컨트롤러 (Utilities|Casting|CastToPlayerController Interactor))))

(event Custom|Event%20Multiple%20Press
  ;[0 0 0 0.426 22] [On Interaction Button Pressed]
  ;
  ; 1. Event Pre Interaction is called from the Player Controller
  ; 2. Before calling 'Event Interaction' check if InputType Holding/Mashing is selected
  ;;[1 0 0 0.2] 2. Check for Input Key Mashing Amount
  (bind _variable (Utilities|MashingInput 10)
    (:then
      (Interaction|FillInteractionWidgetBorder _variable))
    (:Completed
      (Interaction|FillInteractionWidgetBorder _variable)
      (Utilities|FlowControl|Delay 0.2)
      (Class|DELETEBPIObjectInteraction|StartInteractionwithObject(Message) (Variables|Default|GetInteractor) self))))

(event Custom|Event%20Pre%20Interaction
  (params (Interactor :type Actor%20Object%20Reference))
  ;[0 0 0 0.426 22] [On Interaction Button Pressed]
  ;
  ; 1. Event Pre Interaction is called from the Player Controller
  ; 2. Before calling 'Event Interaction' check if InputType Holding/Mashing is selected
  ;;[1 0 0 0.2] 1. On Pre Interaction
  (Variables|Default|SetInteractor Interactor)
  (switch Utilities|FlowControl|Switch|SwitchonEInteractionInputType (Variables|Interaction|GetInput%20Type)
    (:Single
      (Class|DELETEBPIObjectInteraction|StartInteractionwithObject(Message) (Variables|Default|GetInteractor) self))
    (:Holding
      (CallFunction|EventDurationPress))
    (:MultipleANDMashing
      (CallFunction|EventMultiplePress))))

(event Custom|Event%20Duration%20Press
  ;[0 0 0 0.426 22] [On Interaction Button Pressed]
  ;
  ; 1. Event Pre Interaction is called from the Player Controller
  ; 2. Before calling 'Event Interaction' check if InputType Holding/Mashing is selected
  ;;[1 0 0 0.2] 2. Check for Input Key Time Down
  (bind _returnvalue (Utilities|Time|SetTimerbyEvent (delegate Custom|Is%20Key%20Down) 0.05 true))
  (Variables|Interaction|SetKey%20Down%20Timer _returnvalue)
  (bind _key (Utilities|GetPressedKeybyActionName "Interaction")
    (:Valid
      (Variables|Interaction|SetPressed%20Interaction%20Key _key))
    (:Not%20Valid
      (Variables|Interaction|SetPressed%20Interaction%20Key "E"))))

(event Custom|Event%20Initialize
  ;[0 0 0 0.426 22] [On Begin Play]
  ;
  ; 1. Initialize Event is called inside Component Owner [Interactable Object]
  ; 2. Right after that 'Setup Interactable References' is called from Interactable Object
  ;;[1 0 0 0.2] 1. On Initialize
  (Class|DELETEBPIInteractable|Initialize(Message) (Components|GetOwner)))

(event Custom|Setup%20Interactable%20References
  (params (Interactable%20Area :type Box%20Component%20Object%20Reference) (Interaction%20Widget :type Widget%20Component%20Object%20Reference) (Highlightable%20Objects :type Set%20of%20Primitive%20Component%20Object%20References))
  ;[0 0 0 0.426 22] [On Begin Play]
  ;
  ; 1. Initialize Event is called inside Component Owner [Interactable Object]
  ; 2. Right after that 'Setup Interactable References' is called from Interactable Object
  ;;[1 0 0 0.2] 2. Setup Interactable Object
  (Variables|Default|SetInteractable%20Area Interactable%20Area)
  (Variables|Default|SetInteraction%20Widget Interaction%20Widget)
  (bind _result (Utilities|Set|ToArray Highlightable%20Objects))
  (bind _output_get (Variables|Interaction|SetObjects%20to%20Highlight _result))
  (Collision|SetCollisionResponsetoChannel _output_get "ECC_GameTraceChannel1" "ECR_Block") ; Set Channel to Interactable
)

(event Custom|Is%20Key%20Down
  (bind _interactor (Variables|Default|GetInteractor))
  (bind _current_interactable (CallFunction|DELETEGetCurrentInteractableObject _interactor))
  ;[0 0 0 0.426 22] [On Interaction Button Pressed]
  ;
  ; 1. Event Pre Interaction is called from the Player Controller
  ; 2. Before calling 'Event Interaction' check if InputType Holding/Mashing is selected
  ;;[1 0 0 0.2] 2. Check for Input Key Time Down
  (if (and (Utilities|IsValid _current_interactable) (== _current_interactable self))
    (Utilities|HoldingInput
      (:Complete
        (Utilities|Time|ClearandInvalidateTimerbyHandle (Variables|Interaction|GetKey%20Down%20Timer))
        (Class|DELETEBPIObjectInteraction|StartInteractionwithObject(Message) (Variables|Default|GetInteractor) self))
      (:Reset
        (Utilities|Time|ClearandInvalidateTimerbyHandle (Variables|Interaction|GetKey%20Down%20Timer) :!label _label)))
    (else
      (goto _label))))

(event Custom|Event%20Remove%20Interaction
  ;[0 0 0 0.426 22] [On Remove Interaction]
  ;
  ; Event Called from Player Controller
  ; Event Remove Interaction is called inside the Interactable Object
  ; Set IsInteractable to False and Invalidate Interactable Area
  ; If 'Destroy after Pickup' is marked as True - Destroy the Actor
  ;;[1 0 0 0.2] On Remove Interaction
  (Class|DELETEBPIInteractable|RemoveInteraction(Message) (Components|GetOwner))
  (Variables|Main|SetIsInteractable false)
  (Variables|Default|SetInteractable%20Area 0)
  (if (Variables|Interaction|GetDestroy%20after%20Pickup?)
    (Actor|DestroyActor (Components|GetOwner))))

(event Custom|Event%20Re-Initialize%20Associated%20Actors
  ;[0 0 0 0.426 22] [On Re-Initialize]
  ;
  ; 1. Mainly called from Objects after Playing Animation
  ;  If Response = Temporary - Call Initialize Event [Setup References]
  ;  Switch 'Is Interactable' boolean to True & Set Visibility of Interaction Widget
  ; 2. Re-Initialize each Associated Actor
  ;;[1 0 0 0.2] 2. Fire Event Re-Initialize each Associated Actor
  (bind _keys (Utilities|Map|Keys (Variables|Interaction|GetAssociated%20Interactable%20Actors)))
  (for _array_element _keys
    (Utilities|IsValid _array_element
      (:Is%20Valid
        (Utilities|IsValid (Actor|GetComponentbyClass _array_element "DELETE_AC_Interactable_C")
          (:Is%20Valid
            (Interaction|ToggleCanbeReInitialized (Actor|GetComponentbyClass _array_element "DELETE_AC_Interactable_C") true)
            (CallFunction|EventRe-initialize (Actor|GetComponentbyClass _array_element "DELETE_AC_Interactable_C"))))))))

(event Custom|Event%20Re-initialize
  (bind _interaction_widget_ref (Variables|Interaction|GetInteraction%20Widget%20Ref))
  ;[0 0 0 0.426 22] [On Re-Initialize]
  ;
  ; 1. Mainly called from Objects after Playing Animation
  ;  If Response = Temporary - Call Initialize Event [Setup References]
  ;  Switch 'Is Interactable' boolean to True & Set Visibility of Interaction Widget
  ; 2. Re-Initialize each Associated Actor
  ;;[1 0 0 0.2] 1. On Re-initialize
  (switch Utilities|FlowControl|Switch|SwitchonEInteractionResponse (Variables|Interaction|GetInteractable%20Response)
    (:Temporary
      (if (Variables|Interaction|GetCan%20be%20ReInitialized?)
        (Class|DELETEBPIInteractable|Initialize(Message) (Components|GetOwner))
        (Interaction|ToggleIsInteractable true)
        (Utilities|IsValid _interaction_widget_ref
          (:Is%20Valid
            (Widget|SetVisibility _interaction_widget_ref "Visible")))))))

(event Custom|Event%20Associated%20Actor%20End%20Interaction
  ;[0 0 0 0.426 22] [On End Interaction]
  ;
  ; 1. Called from Player Controller
  ; 2. Optional Event to End Interaction in each Associated Actor
  ;;[1 0 0 0.2] 2. Fire Event End Interaction in each Associated Actor
  (bind _keys (Utilities|Map|Keys (Variables|Interaction|GetAssociated%20Interactable%20Actors)))
  (for _array_element _keys
    (Utilities|IsValid _array_element
      (:Is%20Valid
        (Utilities|IsValid (Actor|GetComponentbyClass _array_element "DELETE_AC_Interactable_C")
          (:Is%20Valid
            (CallFunction|EventEndInteraction (Actor|GetComponentbyClass _array_element "DELETE_AC_Interactable_C") (Variables|Default|GetInteractor))))))))

(event Custom|Event%20End%20Interaction
  (params (Interactor :type Actor%20Object%20Reference))
  ;[0 0 0 0.426 22] [On End Interaction]
  ;
  ; 1. Called from Player Controller
  ; 2. Optional Event to End Interaction in each Associated Actor
  ;;[1 0 0 0.2] 1. On End Interaction
  (Class|DELETEBPIInteractable|EndInteraction(Message) (Components|GetOwner) Interactor))

(event Custom|Event%20Game%20Loaded
  (bind _interaction_widget_ref (Variables|Interaction|GetInteraction%20Widget%20Ref))
  ;[0 0 0 0.426 22] [On Game Loaded]
  ;
  ; Called from Game Instance, after Loading a Game from Save
  ;;[1 0 0 0.2] On Game Loaded
  (Class|DELETEBPIInteractable|GameLoad(Message) (Components|GetOwner))
  (Utilities|IsValid _interaction_widget_ref
    (:Is%20Valid
      (Widget|SetVisibility _interaction_widget_ref "Visible"))))