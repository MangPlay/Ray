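; Blueprint function library of shared helpers for the RPG inventory system, with the asset and its functions all prefixed DELETE.
; Getters fetch the player character, camera, interactables and components such as inventory, equipment, stats, crafting and saving.
; Item array helpers drop invalid classes, then filter by type or sort by type, rarity, value or weight, using bucketing or descending insertion.
; Other helpers grant experience, map gamepad icons and rarity colors, play UI sounds and toggle player 2D capture.
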(fn DELETEGetRPGInventoryPlayerRef
  (bind _asbp_rpginventory_character (Utilities|Casting|CastToBP_RPGInventoryCharacter (Game|GetPlayerCharacter 0))
    (:then
      (return _asbp_rpginventory_character))
    (:CastFailed
      (return 0))))

(fn DELETEGetACCrafting
  (params (Target :type Actor%20Object%20Reference))
  (bind _returnvalue (Actor|GetComponentbyClass Target "/Game/InventorySystem/Blueprints/Components/DELETE_AC_Crafting.DELETE_AC_Crafting_C"))
  (Utilities|IsValid _returnvalue
    (:Is%20Valid
      (return _returnvalue))
    (:Is%20Not%20Valid
      (return 0))))

(fn DELETEGetACInteraction
  (params (Target :type Actor%20Object%20Reference))
  (bind _returnvalue (Actor|GetComponentbyClass Target "/Game/InventorySystem/Blueprints/Components/DELETE_AC_Interaction.DELETE_AC_Interaction_C"))
  (Utilities|IsValid _returnvalue
    (:Is%20Valid
      (return _returnvalue))
    (:Is%20Not%20Valid
      (return 0))))

(fn DELETEGetCurrentInteractableObject
  (params (Target :type Actor%20Object%20Reference))
  (bind _returnvalue (Actor|GetComponentbyClass Target "/Game/InventorySystem/Blueprints/Components/DELETE_AC_Interaction.DELETE_AC_Interaction_C"))
  (bind _current_interactable (Variables|/Game/InventorySystem/Blueprints/Components/DELETE_AC_Interaction.DELETE_AC_Interaction_C|GetCurrent%20Interactable _returnvalue))
  (Utilities|IsValid _returnvalue
    (:Is%20Valid
      (Utilities|IsValid _current_interactable
        (:Is%20Valid
          (return _current_interactable))
        (:Is%20Not%20Valid
          (return 0))))
    (:Is%20Not%20Valid
      (return 0))))

(fn DELETEAddLevelExptoPlayer
  (params (Target :type Actor%20Object%20Reference) (Exp%20to%20Add :type Float%20%28double-precision%29))
  (bind _returnvalue (Actor|GetComponentbyClass Target "/Game/InventorySystem/Blueprints/Components/DELETE_AC_Leveling.DELETE_AC_Leveling_C"))
  (Utilities|IsValid Target
    (:Is%20Valid
      (Utilities|IsValid _returnvalue
        (:Is%20Valid
          (Default|ServerAddLevelExp _returnvalue Exp%20to%20Add))))))

(fn DELETEGetACLeveling
  (params (Target :type Actor%20Object%20Reference))
  (bind _returnvalue (Actor|GetComponentbyClass Target "/Game/InventorySystem/Blueprints/Components/DELETE_AC_Leveling.DELETE_AC_Leveling_C"))
  (Utilities|IsValid _returnvalue
    (:Is%20Valid
      (return _returnvalue))
    (:Is%20Not%20Valid
      (return 0))))

(fn DELETESortItemsbyType
  (params (Data%20Array :type Array%20of%20DELETE%20S%20Item%20Data%20Structures))
  (for _array_element Data%20Array
    (Utilities|DELETEIsItemClassValid? _array_element
      (:Valid
        (Utilities|Array|Add (Utilities|Select :Index (Utilities|GetClassDefaults (Utilities|Struct|BreakDELETE_S_ItemData _array_element)) :None 0 :Armor (LocalVariables|GetArmor) :Weapon (LocalVariables|GetWeapons) :Shield (LocalVariables|GetShields) :Food (LocalVariables|GetFood) :Potion (LocalVariables|GetPotions) :CraftingIngredient (LocalVariables|GetCrIngredients) :QuestItem (LocalVariables|GetQItems) :Other (LocalVariables|GetOther) :Currency (LocalVariables|GetCurrency)) _array_element))))
  ;[0.02042 0 1 0.133] Inventory P1
  (Utilities|Array|AppendArray (LocalVariables|GetSorted) (LocalVariables|GetArmor))
  (Utilities|Array|AppendArray (LocalVariables|GetSorted) (LocalVariables|GetWeapons))
  (Utilities|Array|AppendArray (LocalVariables|GetSorted) (LocalVariables|GetShields))
  ;[0 1 0.8949 0.238] Inventory P2
  (Utilities|Array|AppendArray (LocalVariables|GetSorted) (LocalVariables|GetPotions))
  (Utilities|Array|AppendArray (LocalVariables|GetSorted) (LocalVariables|GetFood))
  ;[1 0.7568 0 0.17] Inventory P3
  (Utilities|Array|AppendArray (LocalVariables|GetSorted) (LocalVariables|GetCrIngredients))
  ;[1 0.3792 0 0.17] Inventory P4
  (Utilities|Array|AppendArray (LocalVariables|GetSorted) (LocalVariables|GetQItems))
  (Utilities|Array|AppendArray (LocalVariables|GetSorted) (LocalVariables|GetOther))
  ;[0 0 0 0.488] Non-Panel
  (Utilities|Array|AppendArray (LocalVariables|GetSorted) (LocalVariables|GetCurrency))
  (return (LocalVariables|GetSorted)))

(fn DELETESortItemsbyRarity
  (params (Data%20Array :type Array%20of%20DELETE%20S%20Item%20Data%20Structures))
  (for _array_element Data%20Array
    (Utilities|DELETEIsItemClassValid? _array_element
      (:Valid
        (Utilities|Array|Add (Utilities|Select :Index (Utilities|GetClassDefaults (Utilities|Struct|BreakDELETE_S_ItemData _array_element)) :None 0 :Common (LocalVariables|GetCommon) :Superior (LocalVariables|GetSuperior) :Epic (LocalVariables|GetEpic) :Legendary (LocalVariables|GetLegendary) :Consumable (LocalVariables|GetConsumable) :Usable (LocalVariables|GetUsable)) _array_element))))
  (Utilities|Array|AppendArray (LocalVariables|GetSorted) (LocalVariables|GetLegendary))
  (Utilities|Array|AppendArray (LocalVariables|GetSorted) (LocalVariables|GetEpic))
  (Utilities|Array|AppendArray (LocalVariables|GetSorted) (LocalVariables|GetSuperior))
  (Utilities|Array|AppendArray (LocalVariables|GetSorted) (LocalVariables|GetCommon))
  (Utilities|Array|AppendArray (LocalVariables|GetSorted) (LocalVariables|GetConsumable))
  (Utilities|Array|AppendArray (LocalVariables|GetSorted) (LocalVariables|GetUsable))
  (return (LocalVariables|GetSorted)))

(fn DELETESortItemsbyValue
  (params (Data%20Array :type Array%20of%20DELETE%20S%20Item%20Data%20Structures))
  (for _array_element Data%20Array
    (Utilities|DELETEIsItemClassValid? _array_element
      (:Valid
        (bind (_array_element_2 _array_index) (Utilities|Array|ForEachLoopwithBreak (LocalVariables|GetSorted) :!label _label)
          (:LoopBody
            (if (> (Utilities|GetClassDefaults (Utilities|Struct|BreakDELETE_S_ItemData _array_element)) (Utilities|GetClassDefaults (Utilities|Struct|BreakDELETE_S_ItemData _array_element_2)))
              (Utilities|FlowControl|Sequence
                (:then_0
                  (LocalVariables|SetFound true)
                  (Utilities|Array|Insert (LocalVariables|GetSorted) _array_element _array_index))
                (:then_1
                  (goto _label Break)))))
          (:Completed
            (if (LocalVariables|GetFound)
              (LocalVariables|SetFound false)
              (else
                (Utilities|Array|Add (LocalVariables|GetSorted) _array_element))))))))
  (return (LocalVariables|GetSorted)))

(fn DELETESortItemsbyWeight
  (params (Data%20Array :type Array%20of%20DELETE%20S%20Item%20Data%20Structures))
  (for _array_element Data%20Array
    (Utilities|DELETEIsItemClassValid? _array_element
      (:Valid
        (bind (_array_element_2 _array_index) (Utilities|Array|ForEachLoopwithBreak (LocalVariables|GetSorted) :!label _label)
          (:LoopBody
            (if (> (Utilities|GetClassDefaults (Utilities|Struct|BreakDELETE_S_ItemData _array_element)) (Utilities|GetClassDefaults (Utilities|Struct|BreakDELETE_S_ItemData _array_element_2)))
              (Utilities|FlowControl|Sequence
                (:then_0
                  (LocalVariables|SetFound true)
                  (Utilities|Array|Insert (LocalVariables|GetSorted) _array_element _array_index))
                (:then_1
                  (goto _label Break)))))
          (:Completed
            (if (LocalVariables|GetFound)
              (LocalVariables|SetFound false)
              (else
                (Utilities|Array|Add (LocalVariables|GetSorted) _array_element))))))))
  (return (LocalVariables|GetSorted)))

(fn DELETEQuickSortItems
  (params (Data%20Array :type Array%20of%20DELETE%20S%20Item%20Data%20Structures))
  (for _array_element Data%20Array
    (Utilities|DELETEIsItemClassValid? _array_element
      (:Valid
        (Utilities|Array|Add (LocalVariables|GetSorted) _array_element))))
  (return (LocalVariables|GetSorted)))

(fn DELETEGetGamepadIcon
  (params (Input :type EGamepadInputs%20Enum :default "FaceButtonBottom"))
  (return (Utilities|Select :Index Input :FaceButtonBottom "/Game/InventorySystem/Textures/Images/UILayout/GamepadIcons/T_Gamepad_A.T_Gamepad_A" :FaceButtonRight "/Game/InventorySystem/Textures/Images/UILayout/GamepadIcons/T_Gamepad_B.T_Gamepad_B" :FaceButtonLeft "/Game/InventorySystem/Textures/Images/UILayout/GamepadIcons/T_Gamepad_X.T_Gamepad_X" :FaceButtonTop "/Game/InventorySystem/Textures/Images/UILayout/GamepadIcons/T_Gamepad_Y.T_Gamepad_Y" :LeftThumbstick "/Game/InventorySystem/Textures/Images/UILayout/GamepadIcons/T_Gamepad_LStick.T_Gamepad_LStick" :LeftThumbstickButton "/Game/InventorySystem/Textures/Images/UILayout/GamepadIcons/T_Gamepad_LStickDown.T_Gamepad_LStickDown" :RightThumbstick "/Game/InventorySystem/Textures/Images/UILayout/GamepadIcons/T_Gamepad_RStick.T_Gamepad_RStick" :RightThumbstickButton "/Game/InventorySystem/Textures/Images/UILayout/GamepadIcons/T_Gamepad_RStickDown.T_Gamepad_RStickDown" :LeftShoulder "/Game/InventorySystem/Textures/Images/UILayout/GamepadIcons/T_Gamepad_LB.T_Gamepad_LB" :RightShoulder "/Game/InventorySystem/Textures/Images/UILayout/GamepadIcons/T_Gamepad_RB.T_Gamepad_RB" :LeftTrigger "/Game/InventorySystem/Textures/Images/UILayout/GamepadIcons/T_Gamepad_LT.T_Gamepad_LT" :RightTrigger "/Game/InventorySystem/Textures/Images/UILayout/GamepadIcons/T_Gamepad_RT.T_Gamepad_RT" :DpadUp "/Game/InventorySystem/Textures/Images/UILayout/GamepadIcons/T_Gamepad_DpadUp.T_Gamepad_DpadUp" :DpadDown "/Game/InventorySystem/Textures/Images/UILayout/GamepadIcons/T_Gamepad_DpadDown.T_Gamepad_DpadDown" :DpadRight "/Game/InventorySystem/Textures/Images/UILayout/GamepadIcons/T_Gamepad_DpadRight.T_Gamepad_DpadRight" :DpadLeft "/Game/InventorySystem/Textures/Images/UILayout/GamepadIcons/T_Gamepad_DpadLeft.T_Gamepad_DpadLeft" :SpecialLeft "/Game/InventorySystem/Textures/Images/UILayout/GamepadIcons/T_Gamepad_ViewButton.T_Gamepad_ViewButton" :SpecialRight "/Game/InventorySystem/Textures/Images/UILayout/GamepadIcons/T_Gamepad_MenuButton.T_Gamepad_MenuButton")))

(fn DELETEPlaySoundonItemDropped
  (Audio|PlaySound2D 0 "/Game/InventorySystem/Sounds/S_Click.S_Click" 1.0 1.0 0.0 0 0))

(fn DELETEPlaySoundonOpeningWidget
  (Audio|PlaySound2D 0 "/Game/InventorySystem/Sounds/S_OpenWidget.S_OpenWidget" 1.0 1.0 0.0 0 0))

(fn DELETEPlaySoundonItemPickedUp
  (Audio|PlaySound2D 0 "/Game/InventorySystem/Sounds/S_Pickup.S_Pickup" 1.0 1.0 0.0 0 0))

(fn DELETEPlaySoundonTabSwitched
  (Audio|PlaySound2D 0 "/Game/InventorySystem/Sounds/S_Switch.S_Switch" 0.6 1.0 0.0 0 0))

(fn DELETEPlaySoundonButtonSwitched
  (Audio|PlaySound2D 0 "/Game/InventorySystem/Sounds/S_Click.S_Click" 1.0 1.0 0.0 0 0))

(fn DELETEPlaySoundonItemCrafted
  (Audio|PlaySound2D 0 "/Game/InventorySystem/Sounds/S_Craft.S_Craft" 1.0 1.0 0.0 0 0))

(fn DELETEPlaySoundonConsumableUsed
  (Audio|PlaySound2D 0 "/Game/InventorySystem/Sounds/S_Click.S_Click" 1.0 1.0 0.0 0 0))

(fn DELETEGetACConsumableBuffs
  (params (Target :type Actor%20Object%20Reference))
  (bind _returnvalue (Actor|GetComponentbyClass Target "/Game/InventorySystem/Blueprints/Components/DELETE_AC_ConsumableBuffs.DELETE_AC_ConsumableBuffs_C"))
  (Utilities|IsValid _returnvalue
    (:Is%20Valid
      (return _returnvalue))
    (:Is%20Not%20Valid
      (return 0))))

(fn DELETEGetAllItemsOfType
  (params (Data%20Array :type Array%20of%20DELETE%20S%20Item%20Data%20Structures) (Item%20Type :type EItemType%20Enum :default "None"))
  (for _array_element Data%20Array
    (Utilities|DELETEIsItemClassValid? _array_element
      (:Valid
        (if (Utilities|Enum|Equal(Enum) (Utilities|GetClassDefaults (Utilities|Struct|BreakDELETE_S_ItemData _array_element)) Item%20Type)
          (Utilities|Array|Add (LocalVariables|GetItems) _array_element)))))
  (return (LocalVariables|GetItems)))

(fn DELETEGetPlayerCamera
  (params (Target :type Actor%20Object%20Reference))
  (bind _returnvalue (Actor|GetComponentbyClass Target "/Script/Engine.CameraComponent"))
  (Utilities|IsValid _returnvalue
    (:Is%20Valid
      (return _returnvalue))
    (:Is%20Not%20Valid
      (return 0))))

(fn DELETEGetRarityColor
  (params (Rarity :type EItemRarity%20Enum :default "None"))
  (return (Utilities|Struct|MakeSlateColor (Utilities|Select :Index Rarity :None "" :Common "(R=0.775822,G=0.775822,B=0.775822,A=1.000000)" :Superior "(R=0.046665,G=0.291771,B=0.149960,A=1.000000)" :Epic "(R=0.361307,G=0.000000,B=0.672443,A=1.000000)" :Legendary "(R=0.564712,G=0.417885,B=0.039546,A=1.000000)" :Consumable "(R=0.054480,G=0.291771,B=0.539480,A=1.000000)" :Usable "(R=0.665387,G=0.274677,B=0.082283,A=1.000000)"))))

(fn DELETEGetPlayerInventory
  (params (Target :type Actor%20Object%20Reference))
  (bind _returnvalue (Actor|GetComponentbyClass Target "/Game/InventorySystem/Blueprints/Components/DELETE_AC_PlayerInventory.DELETE_AC_PlayerInventory_C"))
  (Utilities|IsValid _returnvalue
    (:Is%20Valid
      (return _returnvalue))
    (:Is%20Not%20Valid
      (return 0))))

(fn DELETEGetInventoryfromInteractable
  (params (Interactable :type DELETE%20AC%20Interactable%20Object%20Reference))
  (bind _returnvalue (Components|GetOwner Interactable))
  (bind _returnvalue_2 (Actor|GetComponentbyClass _returnvalue "/Game/InventorySystem/Blueprints/Components/DELETE_AC_InventoryCore.DELETE_AC_InventoryCore_C"))
  (Utilities|IsValid Interactable
    (:Is%20Valid
      (Utilities|IsValid _returnvalue_2
        (:Is%20Valid
          (return true _returnvalue_2))
        (:Is%20Not%20Valid
          _)))
    (:Is%20Not%20Valid
      _))
  (return false 0))

(fn DELETEGetPlayerEquipment
  (params (Target :type Actor%20Object%20Reference))
  (bind _returnvalue (Actor|GetComponentbyClass Target "/Game/InventorySystem/Blueprints/Components/DELETE_AC_PlayerEquipment.DELETE_AC_PlayerEquipment_C"))
  (Utilities|IsValid _returnvalue
    (:Is%20Valid
      (return _returnvalue))
    (:Is%20Not%20Valid
      (return 0))))

(fn DELETEGetACStats
  (params (Target :type Actor%20Object%20Reference))
  (bind _returnvalue (Actor|GetComponentbyClass Target "/Game/InventorySystem/Blueprints/Components/DELETE_AC_Stats.DELETE_AC_Stats_C"))
  (Utilities|IsValid _returnvalue
    (:Is%20Valid
      (return _returnvalue))
    (:Is%20Not%20Valid
      (return 0))))

(fn DELETEStartPlayerCapture2D
  (params (Controller :type Actor%20Object%20Reference))
  (bind _asbp_rpginventory_player_controller (Utilities|Casting|CastToBP_RPGInventoryPlayerController Controller))
  (Default|StartPlayerCapture _asbp_rpginventory_player_controller))

(fn DELETEStopPlayerCapture2D
  (params (Controller :type Actor%20Object%20Reference))
  (bind _asbp_rpginventory_player_controller (Utilities|Casting|CastToBP_RPGInventoryPlayerController Controller))
  (Default|StopPlayerCapture _asbp_rpginventory_player_controller))

(fn DELETEGetACSaving
  (params (Target :type Actor%20Object%20Reference))
  (bind _returnvalue (Actor|GetComponentbyClass Target "/Game/InventorySystem/Blueprints/Components/DELETE_AC_Saving.DELETE_AC_Saving_C"))
  (Utilities|IsValid _returnvalue
    (:Is%20Valid
      (return _returnvalue))
    (:Is%20Not%20Valid
      (return 0))))