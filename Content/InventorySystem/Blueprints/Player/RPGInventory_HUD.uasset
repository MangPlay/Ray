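; RPG inventory HUD Blueprint that owns the main WB_HUD widget and exposes loot bar toggling.
; On BeginPlay it creates the widget for the owning player controller, adding it to that player's screen when multiple local players exist, otherwise to the viewport.
; ShowLootBar and HideLootBar events forward to the stored widget after a validity check.
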(event Custom|Hide%20LootBar
  ;[0 0.8314 1 0.452] Toggle LootBar
  (Utilities|IsValid (Variables|Default|GetHUD%20Ref)
    (:Is%20Valid
      (Class|RayOverlayWidget|HideLootBar (Variables|Default|GetHUD%20Ref)))))

(event Custom|Show%20LootBar
  ;[0 0.8314 1 0.452] Toggle LootBar
  (Utilities|IsValid (Variables|Default|GetHUD%20Ref)
    (:Is%20Valid
      (Class|RayOverlayWidget|ShowLootBar (Variables|Default|GetHUD%20Ref)))))

(event EventBeginPlay
  ;[1 0 0.0296 0.53] On Begin Play
  (bind _returnvalue (UserInterface|CreateWidget "/Game/InventorySystem/UI/HUD/WB_HUD.WB_HUD_C" (Game|Player|GetOwningPlayerController)))
  (Variables|Default|SetHUD%20Ref _returnvalue)
  (if (Class|KismetSystemLibrary|HasMultipleLocalPlayers)
    (UserInterface|Viewport|AddtoPlayerScreen (Variables|Default|GetHUD%20Ref))
    (else
      (UserInterface|Viewport|AddtoViewport (Variables|Default|GetHUD%20Ref) 0))))

(fn ConstructionScript)