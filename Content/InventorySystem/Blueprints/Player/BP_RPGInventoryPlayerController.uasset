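; Player controller for the RPG inventory system, routing input, UI state and object interaction to inventory, equipment, crafting, saving and other components.
; On possess it initializes those systems and the player capture actor.
; It tracks active widget, tab, popup and gamepad-versus-mouse mode, gating most gameplay inputs while a main widget is open.
; Interactions pass through client/server events, registering players as viewers of replicated inventories; many DELETE-prefixed members appear slated for removal.
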(event Custom|Initialize%20Components
  ;[0.5938 0 0.004973 0.499 25] Initialize Components [On Possess]
  (CallFunction|InitializePlayerCapture)
  (Default|DELETEInitializeStats (Variables|Default|GetAC_Stats))
  (Default|DELETEInitializeInventory (Variables|Default|GetAC_PlayerInventory))
  (Default|InitializeEquipment (Variables|Default|GetAC_PlayerEquipment))
  (Default|InitializeInteraction (Variables|Default|GetAC_Interaction)))

(event Custom|Initialize%20Player%20Capture
  ;[0.5938 0 0.004973 0.499 25] Client: Initialize Player Capture
  (bind _returnvalue (Actor|GetActorOfClass "/Script/Ray.PlayerCapture"))
  (bind _output_get (Variables|Default|SetPlayerCapture _returnvalue))
  (Utilities|IsValid 0
    (:Is%20Valid
      (Class|PlayerCapture|InitializePlayerCapture _output_get))))

(event Custom|Stop%20Player%20Capture
  ;[0.03125 0.03125 0.03125 0.488 20] Event Start/Stop Player Capture 2D
  (Utilities|IsValid (Variables|Default|GetPlayerCapture)
    (:Is%20Valid
      (Class|PlayerCapture|EventStartCapture (Variables|Default|GetPlayerCapture)))))

(event Custom|Start%20Player%20Capture
  ;[0.03125 0.03125 0.03125 0.488 20] Event Start/Stop Player Capture 2D
  (Utilities|IsValid (Variables|Default|GetPlayerCapture)
    (:Is%20Valid
      (Class|PlayerCapture|EventStartCapture (Variables|Default|GetPlayerCapture)))))

(event EventPossess
  (params (PossessedPawn :type Pawn%20Object%20Reference))
  ;[0.5972 0 0.004777 0.498 24] On Possess/UnPossess InventoryCharacter
  (|CallParentFunction PossessedPawn)
  (CallFunction|InitializeComponents)
  (Utilities|Casting|CastToBP_RPGInventoryCharacter PossessedPawn)
  (Components|Activation|Activate (Variables|Default|GetAC_Interaction) true))

(event EventUnPossess
  (params (UnpossessedPawn :type Pawn%20Object%20Reference))
  ;[0.5972 0 0.004777 0.498 24] On Possess/UnPossess InventoryCharacter
  (|CallParentFunction UnpossessedPawn)
  (Utilities|Casting|CastToBP_RPGInventoryCharacter UnpossessedPawn)
  (Components|Activation|Deactivate (Variables|Default|GetAC_Interaction)))

(event EventBeginPlay
  ;[0.5938 0 0.004973 0.499 25] Begin Play
  (|CallParentFunction))

(fn ConstructionScript)

(fn EndInteraction
  (params (Interactable :type DELETE%20AC%20Interactable%20Object%20Reference))
  (Utilities|IsValid Interactable
    (:Is%20Valid
      (bind _output_get (LocalVariables|SetL%20Object (Components|GetOwner Interactable)))
      (Utilities|IsValid (Actor|GetComponentbyClass _output_get "/Game/InventorySystem/Blueprints/Components/DELETE_AC_InventoryCore.DELETE_AC_InventoryCore_C")
        (:Is%20Valid
          (Default|DELETERemoveViewer (Variables|Default|GetAC_PlayerInventory) (Variables|GetPlayerState) (Actor|GetComponentbyClass _output_get "/Game/InventorySystem/Blueprints/Components/DELETE_AC_InventoryCore.DELETE_AC_InventoryCore_C")))
        (:Is%20Not%20Valid
          _))
      (Default|EventEndInteraction Interactable self))))

(fn StartInteraction
  (params (Interactable :type DELETE%20AC%20Interactable%20Object%20Reference))
  (bind _returnvalue (Components|GetOwner Interactable))
  (Utilities|IsValid Interactable
    (:Is%20Valid
      (Default|EventInteraction Interactable self)
      (Utilities|IsValid Interactable
        (:Is%20Valid
          (Utilities|IsValid _returnvalue
            (:Is%20Valid
              (bind _output_get (LocalVariables|SetL%20Object _returnvalue))
              (Utilities|IsValid (Actor|GetComponentbyClass _output_get "/Game/InventorySystem/Blueprints/Components/DELETE_AC_InventoryCore.DELETE_AC_InventoryCore_C")
                (:Is%20Valid
                  (if (Variables|/Script/Engine.ActorComponent|GetbReplicates (Actor|GetComponentbyClass _output_get "/Game/InventorySystem/Blueprints/Components/DELETE_AC_InventoryCore.DELETE_AC_InventoryCore_C"))
                    (Default|DELETEServerUpdateItems (Variables|Default|GetAC_PlayerInventory) (LocalVariables|GetL%20Object))
                    (Default|DELETEAddViewer (Variables|Default|GetAC_PlayerInventory) (Variables|GetPlayerState) (Actor|GetComponentbyClass _output_get "/Game/InventorySystem/Blueprints/Components/DELETE_AC_InventoryCore.DELETE_AC_InventoryCore_C"))))))))))))

(fn RemoveInteraction
  (params (Interactable :type DELETE%20AC%20Interactable%20Object%20Reference))
  (Utilities|IsValid Interactable
    (:Is%20Valid
      (Default|EventRemoveInteraction Interactable))))

(fn InitializeInteraction
  (params (Interactable :type DELETE%20AC%20Interactable%20Object%20Reference))
  (Utilities|IsValid Interactable
    (:Is%20Valid
      (Default|EventPreInteraction Interactable self))))

(fn IsAnyMainWidgetOpen?
  (if (Utilities|Enum|NotEqual(Enum) (Variables|UIManager|GetActive%20Widget) "None")
    (return true)
    (else
      (return false))))

(fn DELETEGetActivePopUp
  (return (Variables|UIManager|GetActive%20Pop%20up)))

(fn DELETEGetActiveTab
  (return (Variables|UIManager|GetActive%20Tab)))

(fn DELETEGetActiveWidget
  (return (Variables|UIManager|GetActive%20Widget)))

(fn DELETEGetPlayerCapture
  (return (Variables|Default|GetPlayerCapture)))

(fn DELETEGetRPGInventoryController
  (return self))

(event EventDELETEOpenNewWidget
  (params (Widget :type EWidgetType%20Enum :default "None"))
  ;[0.004252 1 0 0.42] Open Widget
  (switch Utilities|FlowControl|Switch|SwitchonEWidgetType Widget
    (:Inventory
      (Default|OpenInventoryWidget (Variables|Default|GetAC_PlayerInventory)))
    (:Crafting
      (Default|DELETEOpenCraftingWidget (Variables|Default|GetAC_Crafting)))
    (:Vendor
      (Default|OpenVendorWidget (Variables|Default|GetAC_PlayerInventory)))
    (:Storage
      (Default|OpenStorageWidget (Variables|Default|GetAC_PlayerInventory)))
    (:LoadGame
      (Default|OpenLoadGameWidget (Variables|Default|GetAC_Saving)))))

(event EventDELETECloseActiveWidget
  ;[0.9323 0 0 0.582] Close Widget
  (switch Utilities|FlowControl|Switch|SwitchonEWidgetType (Variables|UIManager|GetActive%20Widget)
    (:Inventory
      (Default|CloseInventoryWidget (Variables|Default|GetAC_PlayerInventory)))
    (:Crafting
      (Default|DELETECloseCraftingWidget (Variables|Default|GetAC_Crafting)))
    (:Vendor
      (Default|CloseVendorWidget (Variables|Default|GetAC_PlayerInventory)))
    (:Storage
      (Default|CloseStorageWidget (Variables|Default|GetAC_PlayerInventory)))
    (:LoadGame
      (Default|CloseLoadGameWidget (Variables|Default|GetAC_Saving)))))

(event EventDELETECloseActivePopUp
  (bind _pop_up_ref (Variables|UIManager|GetPop%20up%20Ref))
  ;[0.7393 0 1 0.446] Close Active Pop up
  (Variables|UIManager|SetActive%20Pop%20up "None")
  (Utilities|IsValid _pop_up_ref
    (:Is%20Valid
      (Widget|RemovefromParent _pop_up_ref))))

(event EventDELETEOpenSplitStackPopUp
  (params (Item%20Data :type DELETE%20S%20Item%20Data%20Structure) (InSlot%20Data :type DELETE%20S%20Item%20Data%20Structure) (Sender :type DELETE%20AC%20Inventory%20Core%20Object%20Reference) (Receiver :type DELETE%20AC%20Inventory%20Core%20Object%20Reference) (Input%20Method :type EInputMethod%20Enum :default "RightClick") (Initiator :type EItemDestination%20Enum :default "None") (Destination :type EItemDestination%20Enum :default "None") (Sender%20Widget :type User%20Widget%20Object%20Reference))
  ;[0.7393 0 1 0.446] Open Split Stack Pop up
  (bind _returnvalue (UserInterface|CreateWidget "/Game/InventorySystem/UI/PlayerInventory/WBP_SplitStack.WBP_SplitStack_C" self Item%20Data InSlot%20Data Sender Receiver Input%20Method Initiator Sender%20Widget Destination))
  (Variables|UIManager|SetPop%20up%20Ref _returnvalue)
  (if (not (Class|KismetSystemLibrary|HasMultipleLocalPlayers))
    (UserInterface|Viewport|AddtoViewport (Variables|UIManager|GetPop%20up%20Ref) 1)
    (else
      (UserInterface|Viewport|AddtoPlayerScreen (Variables|UIManager|GetPop%20up%20Ref) 1)))
  (Widget|SetKeyboardFocus (Variables|UIManager|GetPop%20up%20Ref))
  (Variables|UIManager|SetActive%20Pop%20up "SplitStackPopup"))

(event EventDELETEOpenConfirmationPopUp
  (params (Question%20Text :type Text) (Item%20Data :type DELETE%20S%20Item%20Data%20Structure) (InSlot%20Data :type DELETE%20S%20Item%20Data%20Structure) (Sender :type DELETE%20AC%20Inventory%20Core%20Object%20Reference) (Receiver :type DELETE%20AC%20Inventory%20Core%20Object%20Reference) (Input%20Method :type EInputMethod%20Enum :default "RightClick") (Initiator :type EItemDestination%20Enum :default "None") (Destination :type EItemDestination%20Enum :default "None") (Sender%20Widget :type User%20Widget%20Object%20Reference))
  ;[0.7393 0 1 0.446] Open Confirmation Pop up
  (bind _returnvalue (UserInterface|CreateWidget "/Game/InventorySystem/UI/PlayerInventory/WBP_ConfirmationPopup.WBP_ConfirmationPopup_C" self Question%20Text Item%20Data InSlot%20Data Sender Receiver Input%20Method Initiator Destination Sender%20Widget))
  (Variables|UIManager|SetPop%20up%20Ref _returnvalue)
  (if (not (Class|KismetSystemLibrary|HasMultipleLocalPlayers))
    (UserInterface|Viewport|AddtoViewport (Variables|UIManager|GetPop%20up%20Ref) 1)
    (else
      (UserInterface|Viewport|AddtoPlayerScreen (Variables|UIManager|GetPop%20up%20Ref) 1)))
  (Widget|SetKeyboardFocus (Variables|UIManager|GetPop%20up%20Ref))
  (Variables|UIManager|SetActive%20Pop%20up "ConfirmationPopup"))

(event EventDELETEOpenTextDocumentPopUp
  (params (Item%20Data :type DELETE%20S%20Item%20Data%20Structure) (Sender%20Widget :type User%20Widget%20Object%20Reference))
  ;[0.7393 0 1 0.446] Open Text Document Pop up
  (bind _returnvalue (UserInterface|CreateWidget "/Game/InventorySystem/UI/PlayerInventory/WBP_TextDocument.WBP_TextDocument_C" self Item%20Data Sender%20Widget))
  (Variables|UIManager|SetPop%20up%20Ref _returnvalue)
  (if (not (Class|KismetSystemLibrary|HasMultipleLocalPlayers))
    (UserInterface|Viewport|AddtoViewport (Variables|UIManager|GetPop%20up%20Ref) 1)
    (else
      (UserInterface|Viewport|AddtoPlayerScreen (Variables|UIManager|GetPop%20up%20Ref) 1)))
  (Widget|SetKeyboardFocus (Variables|UIManager|GetPop%20up%20Ref))
  (Variables|UIManager|SetActive%20Pop%20up "TextDocumentPopup"))

(event EventDELETESetActiveWidget
  (params (Widget :type EWidgetType%20Enum :default "None"))
  ;[1 0.8148 0 0.451] Set Active Widget / Tab
  (bind _output_get (Variables|UIManager|SetActive%20Widget Widget))
  (Default|CallOnSwitchedWidget _output_get))

(event EventDELETESetActiveTab
  (params (Tab :type EWidgetType%20Enum :default "None"))
  ;[1 0.8148 0 0.451] Set Active Widget / Tab
  (bind _output_get (Variables|UIManager|SetActive%20Tab Tab))
  (Default|CallOnSwitchedTab _output_get))

(event EventDELETESwitchWidgetto
  (params (New%20Widget :type EWidgetType%20Enum :default "None"))
  ;[1 0.8148 0 0.451] Switch Widget to
  (if (Utilities|Enum|NotEqual(Enum) New%20Widget (Variables|UIManager|GetActive%20Widget))
    (CallFunction|DELETECloseActiveWidget)
    (CallFunction|DELETEOpenNewWidget New%20Widget)))

(event EventDELETESwitchTabto
  (params (New%20Tab :type EWidgetType%20Enum :default "None"))
  ;[1 0.8148 0 0.451] Switch Tab to
  (if (Utilities|Enum|NotEqual(Enum) New%20Tab (Variables|UIManager|GetActive%20Tab))
    (CallFunction|DELETESetActiveTab New%20Tab)))

(event EventDELETEDisplayMessageNotify
  (params (Message :type Text))
  ;[1 0 0.3392 0.467] Display Notification Message
  (bind _foundwidgets (Widget|GetAllWidgetsOfClass "/Game/InventorySystem/UI/Misc/Pop-upWidgets/WB_PopupMessage.WB_PopupMessage_C" true)) ; Is Any Message already being displayed?
  (if (== (Utilities|Array|Length _foundwidgets) 0)
    (bind _returnvalue (UserInterface|CreateWidget "/Game/InventorySystem/UI/Misc/Pop-upWidgets/WB_PopupMessage.WB_PopupMessage_C" self Message))
    (if (not (Class|KismetSystemLibrary|HasMultipleLocalPlayers))
      (UserInterface|Viewport|AddtoViewport _returnvalue 1)
      (else
        (UserInterface|Viewport|AddtoPlayerScreen _returnvalue 1)))))

(event EventSetGamepadControls
  (params (IsGamepad :type Boolean))
  ;[0.01033 0.01033 0.01033 0.2196] Toggle Gamepad Controls
  (if (Math|Boolean|NotEqual(Boolean) IsGamepad (Variables|Gamepad|GetGamepadControls))
    (bind _output_get (Variables|Gamepad|SetGamepadControls IsGamepad))
    (Default|CallOnGamepadToggled _output_get)
    (if (Variables|Gamepad|GetGamepadControls)
      (Class|PlayerController|SetMouseLocation))))

(event EventSetCurrentlyFocusedWidget
  (params (Widget :type EWidgetType%20Enum :default "None"))
  ;[0.01033 0.01033 0.01033 0.2196] Set Currently Focused Widget
  (if (Utilities|Enum|NotEqual(Enum) Widget (Variables|Gamepad|GetFocused%20Widget))
    (Variables|Gamepad|SetFocused%20Widget Widget)
    (Default|CallOnFocusedNewWidget)))

(event Input|MouseEvents|MouseX
  (params (AxisValue :type Float%20%28single-precision%29))
  ;[0.01033 0.01033 0.01033 0.2196] Check for Mouse Axis
  (if (or (!= AxisValue 0.0) (!= (stale Input|MouseEvents|MouseY AxisValue) 0.0))
    (CallFunction|SetGamepadControls false)))

(event Input|MouseEvents|MouseY
  (params (AxisValue :type Float%20%28single-precision%29))
  ;[0.01033 0.01033 0.01033 0.2196] Check for Mouse Axis
  (if (or (!= (stale Input|MouseEvents|MouseX AxisValue) 0.0) (!= AxisValue 0.0))
    (CallFunction|SetGamepadControls false)))

(event Input|KeyboardEvents|AnyKey
  (params (Key :type Key%20Structure))
  ;[0.01033 0.01033 0.01033 0.2196] Check for Gamepad
  (:Pressed
    (CallFunction|SetGamepadControls (Class|KismetInputLibrary|KeyIsGamepadKey Key))))

(event Custom|Server%20Remove%20Interaction%20from%20Object
  (params (Interactable :type DELETE%20AC%20Interactable%20Object%20Reference))
  ;[0.776 0 0.119 0.499 25] SERVER: Remove Interaction from Object [RemoveInteraction]
  (Interaction|RemoveInteraction Interactable))

(event Custom|Client%20Initialize%20Interaction%20with%20Object
  (params (Interactable :type DELETE%20AC%20Interactable%20Object%20Reference))
  ;[0.5 0 1 0.551 25] CLIENT: Initialize Interaction with Object [PreInteraction]
  (Interaction|InitializeInteraction Interactable))

(event Custom|Server%20Start%20Interaction%20with%20Object
  (params (Interactable :type DELETE%20AC%20Interactable%20Object%20Reference))
  ;[0 0.6458 0.0509 0.556 25] SERVER: Start Interaction with Object [Interaction]
  (Interaction|StartInteraction Interactable))

(event Custom|Server%20End%20Interaction%20with%20Object
  (params (Interactable :type DELETE%20AC%20Interactable%20Object%20Reference))
  ;[0.7969 0.4383 0 0.478 25] SERVER: End Interaction with Object [EndInteraction]
  (Interaction|EndInteraction Interactable))

(event EventStartInteractionwithObject
  (params (Interactable :type DELETE%20AC%20Interactable%20Object%20Reference))
  ;[0 0.6458 0.0509 0.556 25] SERVER: Start Interaction with Object [Interaction]
  (Utilities|IsValid Interactable
    (:Is%20Valid
      (CallFunction|ServerStartInteractionwithObject Interactable))))

(event EventEndInteractionwithObject
  (params (Interactable :type DELETE%20AC%20Interactable%20Object%20Reference))
  ;[0.7969 0.4383 0 0.478 25] SERVER: End Interaction with Object [EndInteraction]
  (Utilities|IsValid Interactable
    (:Is%20Valid
      (CallFunction|ServerEndInteractionwithObject Interactable))))

(event EventRemoveInteractionfromObject
  (params (Interactable :type DELETE%20AC%20Interactable%20Object%20Reference))
  ;[0.776 0 0.119 0.499 25] SERVER: Remove Interaction from Object [RemoveInteraction]
  (Utilities|IsValid Interactable
    (:Is%20Valid
      (CallFunction|ServerRemoveInteractionfromObject Interactable))))

(event EventInitializeInteractionwithObject
  (params (Interactable :type DELETE%20AC%20Interactable%20Object%20Reference))
  ;[0.5 0 1 0.551 25] CLIENT: Initialize Interaction with Object [PreInteraction]
  (Utilities|IsValid Interactable
    (:Is%20Valid
      (CallFunction|ClientInitializeInteractionwithObject Interactable))))

(event Input|ActionEvents|InputActionCloseWidget
  (params (Key :type Key%20Structure))
  ;[0 0.7454 0.4179 0.298 24] Main Inputs
  (:Pressed
    (Default|InputCloseWidget (Variables|Default|GetAC_PlayerInventory))))

(event Input|ActionEvents|InputActionLoadGame
  (params (Key :type Key%20Structure))
  ;[0 0.7454 0.4179 0.298] Save/Load Inputs
  (:Pressed
    (Default|InputLoadGame (Variables|Default|GetAC_Saving))))

(event Input|ActionEvents|InputActionInteraction
  (params (Key :type Key%20Structure))
  ;[0 0.7454 0.4179 0.298 24] Main Inputs
  (:Pressed
    (if (not (CallFunction|IsAnyMainWidgetOpen?))
      (Default|InputInteraction (Variables|Default|GetAC_PlayerInventory)))))

(event Input|ActionEvents|InputActionInventory
  (params (Key :type Key%20Structure))
  ;[0 0.7454 0.4179 0.298 24] Main Inputs
  (:Pressed
    (Default|InputInventory (Variables|Default|GetAC_PlayerInventory))))

(event Input|ActionEvents|InputActionTakeAllLoot
  (params (Key :type Key%20Structure))
  ;[0 0.7454 0.4179 0.298 24] Main Inputs
  (:Pressed
    (if (not (CallFunction|IsAnyMainWidgetOpen?))
      (Default|InputTakeAll (Variables|Default|GetAC_PlayerInventory)))))

(event Input|ActionEvents|InputActionUsePocket1
  (params (Key :type Key%20Structure))
  ;[0 0.7454 0.4179 0.298] Pocket Inputs
  (:Released
    (if (not (CallFunction|IsAnyMainWidgetOpen?))
      (Default|OnUsePocket1 (Variables|Default|GetAC_ConsumableBuffs)))))

(event Input|ActionEvents|InputActionUsePocket2
  (params (Key :type Key%20Structure))
  ;[0 0.7454 0.4179 0.298] Pocket Inputs
  (:Released
    (if (not (CallFunction|IsAnyMainWidgetOpen?))
      (Default|OnUsePocket2 (Variables|Default|GetAC_ConsumableBuffs)))))

(event Input|ActionEvents|InputActionUsePocket3
  (params (Key :type Key%20Structure))
  ;[0 0.7454 0.4179 0.298] Pocket Inputs
  (:Released
    (if (not (CallFunction|IsAnyMainWidgetOpen?))
      (Default|OnUsePocket3 (Variables|Default|GetAC_ConsumableBuffs)))))

(event Input|ActionEvents|InputActionUsePocket4
  (params (Key :type Key%20Structure))
  ;[0 0.7454 0.4179 0.298] Pocket Inputs
  (:Released
    (if (not (CallFunction|IsAnyMainWidgetOpen?))
      (Default|OnUsePocket4 (Variables|Default|GetAC_ConsumableBuffs)))))

(event Input|ActionEvents|InputActionQuicksave
  (params (Key :type Key%20Structure))
  ;[0 0.7454 0.4179 0.298] Save/Load Inputs
  (:Released
    (if (not (CallFunction|IsAnyMainWidgetOpen?))
      (Default|QuickSaveGame (Variables|Default|GetAC_Saving)))))

(fn GetCurrentlyFocusedWidget
  (return (Variables|Gamepad|GetFocused%20Widget)))

(fn GetInventoryController
  (return 0))

(fn IsUsingGamepad?
  (return (Variables|Gamepad|GetGamepadControls)))