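; BP_TriggerType02 is an interactable trigger, part of the inventory system, whose mesh spins on roll when used.
; Server-side interaction plays or reverses a timeline based on the interactable component's value, then changes that value and notifies associated actors.
; The timeline updates MeshRotation, which its OnRep applies to the mesh, and can reinitialize the interactable on finishing.
; Construction script derives timeline play rate from Duration.
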(event Custom|Move%20Forward
  ;[1 0.02708 0 0.18] MULTICAST: Rotate Mesh
  (bind _newtrack_0 (Timeline|Timeline_0 Play)
    (:Update
      (Variables|Default|SetMesh%20Rotation (Math|Rotator|Lerp(Rotator) "0, 0, 0" (Math|Rotator|MakeRotator (* (Variables|Default|GetRotation%20Amount) (Math|Float|MakeLiteralFloat 3.6e+02)) 0.0 0.0) _newtrack_0)))
    (:Finished
      (if (Variables|Default|GetRe-initialize%20on%20Moving%20Finished)
        (Default|EventRe-initialize (Variables|Default|GetAC_Interactable))))))

(event Custom|Move%20Backward
  ;[1 0.02708 0 0.18] MULTICAST: Rotate Mesh
  (bind _newtrack_0 (Timeline|Timeline_0 Reverse)
    (:Update
      (Variables|Default|SetMesh%20Rotation (Math|Rotator|Lerp(Rotator) "0, 0, 0" (Math|Rotator|MakeRotator (* (Variables|Default|GetRotation%20Amount) (Math|Float|MakeLiteralFloat 3.6e+02)) 0.0 0.0) _newtrack_0)))
    (:Finished
      (if (Variables|Default|GetRe-initialize%20on%20Moving%20Finished)
        (Default|EventRe-initialize (Variables|Default|GetAC_Interactable))))))

(event EventInitialize
  ;[0 0 0 0.227 22] On Initialize
  (Default|SetupInteractableReferences (Variables|Default|GetAC_Interactable) (Variables|Default|GetInteractableArea) (Variables|Default|GetInteractionWidget) (Utilities|Set|MakeSet (Variables|Default|GetStaticMesh))))

(event EventRemoveInteraction
  ;[0 0 0 0.227 22] On Remove Interaction
)

(event EventGameLoad
  ;[0 0 0 0.227 22] On Game Load
)

(event EventInteraction
  (params (Interactor :type Actor%20Object%20Reference))
  ;[0 0 0 0.227 22] SERVER: On Interaction
  (Utilities|IsValid Interactor
    (:Is%20Valid
      (bind _output_get (Variables|Default|SetInteractor 0))
      (Actor|SetOwner _output_get)
      (Utilities|FlowControl|Sequence
        (:then_0
          (switch int (Variables|/Game/InventorySystem/Blueprints/Components/DELETE_AC_Interactable.DELETE_AC_Interactable_C|GetInteractable%20Value (Variables|Default|GetAC_Interactable))
            (:0
              (CallFunction|MoveForward))
            (:1
              (CallFunction|MoveBackward))))
        (:then_1
          (Default|ChangeInteractableValue (Variables|Default|GetAC_Interactable) true)
          (Default|EventAssociatedActorInteraction (Variables|Default|GetAC_Interactable) (Variables|Default|GetInteractor)))))))

(event EventEndInteraction
  (params (Interactor :type Actor%20Object%20Reference))
  ;[0 0 0 0.227 22] On End Interaction
)

(fn ConstructionScript
  (Components|Timeline|SetPlayRate (Variables|Default|GetTimeline_0) (/ 1.0 (Variables|Default|GetDuration))))

(fn OnRepMeshRotation
  (Transformation|SetRelativeRotation (Variables|Default|GetStaticMesh) (Variables|Default|GetMesh%20Rotation) false false))