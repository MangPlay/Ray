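; BP_ElevatorType01 is an interactable elevator that travels between its initial transform and a destination point as pawns step on and off.
; Overlaps on InteractableArea start or end interaction through the pawn's controller; it moves forward for the first occupant and backward when the area empties.
; Travel updates lerp the actor transform and store timeline playback position in ACInteractable, which game load uses to restore position.
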(event OnComponentBeginOverlap(InteractableArea)
  (params (OverlappedComponent :type Primitive%20Component%20Object%20Reference) (OtherActor :type Actor%20Object%20Reference) (OtherComp :type Primitive%20Component%20Object%20Reference) (OtherBodyIndex :type Integer) (bFromSweep :type Boolean) (SweepResult :type Hit%20Result%20Structure%20%28by%20ref%29))
  ;[1 0 0.03031 0.238 22] On Player Begin/End Overlap
  (bind _as폰 (Utilities|Casting|CastToPawn OtherActor))
  (Class|DELETEBPIObjectInteraction|StartInteractionwithObject(Message) (Pawn|GetController _as폰) (Variables|Default|GetAC_Interactable)))

(event OnComponentEndOverlap(InteractableArea)
  (params (OverlappedComponent :type Primitive%20Component%20Object%20Reference) (OtherActor :type Actor%20Object%20Reference) (OtherComp :type Primitive%20Component%20Object%20Reference) (OtherBodyIndex :type Integer))
  ;[1 0 0.03031 0.238 22] On Player Begin/End Overlap
  (bind _as폰 (Utilities|Casting|CastToPawn OtherActor))
  (Class|DELETEBPIObjectInteraction|EndInteractionwithObject(Message) (Pawn|GetController _as폰) (Variables|Default|GetAC_Interactable)))

(event EventInteraction
  (params (Interactor :type Actor%20Object%20Reference))
  ;[0 0 0 0.227 22] SERVER: On Interaction
  (Utilities|IsValid Interactor
    (:Is%20Valid
      (bind _output_get (Variables|Default|SetInteractor Interactor))
      (Actor|SetOwner _output_get)
      (if (<= (Utilities|Array|Length (Collision|GetOverlappingActors (Variables|Default|GetInteractableArea) "/Script/Engine.Pawn" :!class /Script/Engine.PrimitiveComponent)) 1) ; Someone already overlapping?
        (CallFunction|MoveForward)))))

(event EventInitialize
  ;[0 0 0 0.227 22] On Initialize
  (Default|SetupInteractableReferences (Variables|Default|GetAC_Interactable) (Variables|Default|GetInteractableArea) (Variables|Default|GetInteractionWidget) (Utilities|Set|MakeSet)))

(event EventRemoveInteraction
  ;[0 0 0 0.227 22] On Remove Interaction
)

(event EventGameLoad
  ;[0 0 0 0.227 22] On Game Load
  (CallFunction|SetTimelinePostion (Variables|/Game/InventorySystem/Blueprints/Components/DELETE_AC_Interactable.DELETE_AC_Interactable_C|GetTimeline%20Position (Variables|Default|GetAC_Interactable))))

(event EventEndInteraction
  (params (Interactor :type Actor%20Object%20Reference))
  ;[0 0 0 0.227 22] SERVER: On Interaction
  (Utilities|IsValid Interactor
    (:Is%20Valid
      (bind _output_get (Variables|Default|SetInteractor Interactor))
      (Actor|SetOwner _output_get)
      (if (<= (Utilities|Array|Length (Collision|GetOverlappingActors (Variables|Default|GetInteractableArea) "/Script/Engine.Pawn" :!class /Script/Engine.PrimitiveComponent)) 0)
        (CallFunction|MoveBackward)))))

(fn ConstructionScript)

(fn UpdateTravelTransform
  (params (Current%20Time :type Float%20%28double-precision%29))
  (bind _ac_interactable (Variables|Default|GetAC_Interactable))
  (bind _destination_point (Variables|/Game/InventorySystem/Blueprints/Components/DELETE_AC_Interactable.DELETE_AC_Interactable_C|GetDestination%20Point _ac_interactable))
  (Utilities|IsValid _destination_point
    (:Is%20Valid
      (Transformation|SetActorTransform (Math|Transform|Lerp(Transform) (Variables|Default|GetInitial%20Transform) (Transformation|GetActorTransform _destination_point) Current%20Time))
      (Variables|/Game/InventorySystem/Blueprints/Components/DELETE_AC_Interactable.DELETE_AC_Interactable_C|SetTimeline%20Position (Variables|Default|GetAC_Interactable) (Components|Timeline|GetPlaybackPosition (Variables|Default|GetTimeline_ObjectTransform))))))

(fn UnPauseTimeline
  (if (Collision|IsOverlappingActor (Variables|Default|GetInteractableArea) (Game|GetPlayerCharacter 0) :!class /Script/Engine.PrimitiveComponent)
    (CallFunction|MoveForward)
    (elif (Audio|Components|Audio|IsPlaying (Variables|Default|GetTimeline_ObjectTransform))
      (CallFunction|MoveBackward))))