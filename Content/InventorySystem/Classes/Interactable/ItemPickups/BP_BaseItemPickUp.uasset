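; Base item pickup actor for the inventory system, handling player interaction, loot bar display and dropped-item physics.
; Server interaction events set the interactor as owner, then transfer items directly or, when ShowLootBar is enabled, use client events to toggle the prompt and loot bar.
; Removing interaction or destroying the pickup hides both widgets.
; A multicast event enables static mesh physics, ignores Pawn and WorldDynamic, and disables skeletal mesh collision.
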(event Custom|Multicast%20Set%20Physics%20Simulation
  ;[0.0625 0.0625 0.0625 0.587] Multicast Simulate Physics
  (CallFunction|SetPhysicsSimulationandCollision))

(event EventRemoveInteraction
  (bind _local_interactor (Variables|Default|GetLocal%20Interactor))
  (bind _returnvalue (Actor|GetComponentbyClass _local_interactor "/Game/InventorySystem/Blueprints/Components/DELETE_AC_PlayerInventory.DELETE_AC_PlayerInventory_C"))
  ;[1 0.4971 0] On Remove Interaction
  ;[0.2775 0 1 0.305] Toggle Interaction Widget
  (Default|ToggleInteractionWidget (Variables|Default|GetAC_Interactable) false)
  ;[0 1 0.03192 0.52] Get Player Inventory and Close Loot Bar Widget (if 'Show LootBar' was checked)
  (if (Variables|/Game/InventorySystem/Blueprints/Components/DELETE_AC_Interactable.DELETE_AC_Interactable_C|GetShow%20LootBar (Variables|Default|GetAC_Interactable))
    (Utilities|IsValid _local_interactor
      (:Is%20Valid
        (Utilities|IsValid _returnvalue
          (:Is%20Valid
            (Default|CloseLootBarWidget _returnvalue)))))))

(event EventInteraction
  (params (Interactor :type Actor%20Object%20Reference))
  ;[1 0 0.01436 0.248] SERVER: Start/End Interaction Events
  (Utilities|IsValid Interactor
    (:Is%20Valid
      (bind _output_get (Variables|Default|SetInteractor Interactor))
      (Actor|SetOwner _output_get)
      (if (not (Variables|/Game/InventorySystem/Blueprints/Components/DELETE_AC_Interactable.DELETE_AC_Interactable_C|GetShow%20LootBar (Variables|Default|GetAC_Interactable)))
        ;[1 0.103 0 0.305] Bypass Opening LootBar
        (CallFunction|TrytoTransferItems (Variables|Default|GetInteractor))
        (else
          (CallFunction|ClientStartInteraction (Variables|Default|GetInteractor)))))))

(event EventDestroyed
  (bind _local_interactor (Variables|Default|GetLocal%20Interactor))
  (bind _returnvalue (Actor|GetComponentbyClass _local_interactor "/Game/InventorySystem/Blueprints/Components/DELETE_AC_PlayerInventory.DELETE_AC_PlayerInventory_C"))
  ;[1 0.4971 0] On Remove Interaction
  ;[0.2775 0 1 0.305] Toggle Interaction Widget
  (Default|ToggleInteractionWidget (Variables|Default|GetAC_Interactable) false)
  ;[0 1 0.03192 0.52] Get Player Inventory and Close Loot Bar Widget (if 'Show LootBar' was checked)
  (if (Variables|/Game/InventorySystem/Blueprints/Components/DELETE_AC_Interactable.DELETE_AC_Interactable_C|GetShow%20LootBar (Variables|Default|GetAC_Interactable))
    (Utilities|IsValid _local_interactor
      (:Is%20Valid
        (Utilities|IsValid _returnvalue
          (:Is%20Valid
            (Default|CloseLootBarWidget _returnvalue)))))))

(event EventEndInteraction
  (params (Interactor :type Actor%20Object%20Reference))
  ;[1 0 0.01436 0.248] SERVER: Start/End Interaction Events
  (Utilities|IsValid Interactor
    (:Is%20Valid
      (bind _output_get (Variables|Default|SetInteractor Interactor))
      (Actor|SetOwner _output_get)
      (if (Variables|/Game/InventorySystem/Blueprints/Components/DELETE_AC_Interactable.DELETE_AC_Interactable_C|GetShow%20LootBar (Variables|Default|GetAC_Interactable))
        (CallFunction|ClientEndInteraction)))))

(event EventClientStartInteraction
  (params (Interactor :type Actor%20Object%20Reference))
  ;[0 1 0.01898 0.551] CLIENT: Start/End Interaction Events
  (Variables|Default|SetLocal%20Interactor Interactor)
  (Default|ToggleInteractionWidget (Variables|Default|GetAC_Interactable) false)
  (Utilities|IsValid (Actor|GetComponentbyClass (Variables|Default|GetLocal%20Interactor) "/Game/InventorySystem/Blueprints/Components/DELETE_AC_PlayerInventory.DELETE_AC_PlayerInventory_C")
    (:Is%20Valid
      (Default|OpenLootBarWidget (Actor|GetComponentbyClass (Variables|Default|GetLocal%20Interactor) "/Game/InventorySystem/Blueprints/Components/DELETE_AC_PlayerInventory.DELETE_AC_PlayerInventory_C")))))

(event EventClientEndInteraction
  (bind _local_interactor (Variables|Default|GetLocal%20Interactor))
  (bind _returnvalue (Actor|GetComponentbyClass _local_interactor "/Game/InventorySystem/Blueprints/Components/DELETE_AC_PlayerInventory.DELETE_AC_PlayerInventory_C"))
  ;[0 1 0.01898 0.551] CLIENT: Start/End Interaction Events
  (Default|ToggleInteractionWidget (Variables|Default|GetAC_Interactable) true)
  (Utilities|IsValid _local_interactor
    (:Is%20Valid
      (Utilities|IsValid _returnvalue
        (:Is%20Valid
          (Default|CloseLootBarWidget _returnvalue))))))

(fn ConstructionScript
  (|CallParentFunction))

(fn SetPhysicsSimulationandCollision
  (bind _staticmesh (Variables|Default|GetStaticMesh))
  (Physics|SetSimulatePhysics _staticmesh true)
  (Collision|SetCollisionResponsetoChannel _staticmesh "ECC_Pawn" "ECR_Ignore")
  (Collision|SetCollisionResponsetoChannel (Variables|Default|GetStaticMesh) "ECC_WorldDynamic" "ECR_Ignore")
  (Collision|SetCollisionEnabled (Variables|Default|GetSkeletalMesh) "NoCollision"))