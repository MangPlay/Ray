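; BP_Vendor is an interactable vendor actor in the inventory system that opens and closes the interacting player's Vendor widget.
; Server-side interaction events store the Interactor and make it the actor's owner, then call client events.
; The client events switch the Interactor to the Vendor widget on start, and on end close it only if it is still active, through DELETE-prefixed widget-message functions.
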(event EventClientStartInteraction
  (params (Interactor :type Actor%20Object%20Reference))
  ;[0 1 0.01898 0.551] CLIENT: Start/End Interaction Events
  (bind _output_get (Variables|Default|SetInteractor Interactor))
  (Class|DELETEBPIWidgetManager|DELETESwitchWidgetto(Message) _output_get "Vendor"))

(event EventClientEndInteraction
  (bind _interactor (Variables|Default|GetInteractor))
  ;[0 1 0.01898 0.551] CLIENT: Start/End Interaction Events
  (Utilities|IsValid _interactor
    (:Is%20Valid
      (bind _widget (Class|DELETEBPIWidgetManager|DELETEGetActiveWidget(Message) _interactor))
      (if (Utilities|Enum|Equal(Enum) _widget "Vendor")
        (Class|DELETEBPIWidgetManager|DELETECloseActiveWidget(Message) (Variables|Default|GetInteractor))))))

(event EventInteraction
  (params (Interactor :type Actor%20Object%20Reference))
  ;[1 0 0.01436 0.248] SERVER: Start/End Interaction Events
  (Utilities|IsValid Interactor
    (:Is%20Valid
      (bind _output_get (Variables|Default|SetInteractor Interactor))
      (Actor|SetOwner _output_get)
      (CallFunction|ClientStartInteraction (Variables|Default|GetInteractor)))))

(event EventEndInteraction
  (params (Interactor :type Actor%20Object%20Reference))
  ;[1 0 0.01436 0.248] SERVER: Start/End Interaction Events
  (Utilities|IsValid Interactor
    (:Is%20Valid
      (bind _output_get (Variables|Default|SetInteractor Interactor))
      (Actor|SetOwner _output_get)
      (CallFunction|ClientEndInteraction))))

(fn ConstructionScript
  (|CallParentFunction))