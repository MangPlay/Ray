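; Interactable storage chest that opens for an interacting player and shows the Storage widget.
; Server-side Interaction and EndInteraction events set the interactor as owner, then hand off to client events.
; The client hides the prompt, plays the open animation, blocks movement and shows the widget after a short timer.
; Ending clears that timer, closes the chest, restores prompt and movement, and closes the widget if still active.
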(event Custom|Open%20Chest
  ;[1 0.5038 0 0.426] CLIENT: Open/Close Chest
  (if (not (Variables|Default|GetIsOpen))
    (Components|Animation|PlayAnimation (Variables|Default|GetSkeletalMesh) "/Game/InventorySystem/Animations/Chest_Open.Chest_Open" false)
    (Variables|Default|SetIsOpen true)))

(event Custom|Close%20Chest
  ;[1 0.5038 0 0.426] CLIENT: Open/Close Chest
  (if (Variables|Default|GetIsOpen)
    (Components|Animation|PlayAnimation (Variables|Default|GetSkeletalMesh) "/Game/InventorySystem/Animations/Chest_Close.Chest_Close" false)
    (Variables|Default|SetIsOpen false)))

(event Custom|Open%20Widget
  ;[0 1 0.01898 0.551] CLIENT: Start/End Interaction Events
  (Class|DELETEBPIWidgetManager|DELETESwitchWidgetto(Message) (Variables|Default|GetInteractor) "Storage"))

(event EventClientStartInteraction
  (params (Interactor :type Actor%20Object%20Reference))
  ;[0 1 0.01898 0.551] CLIENT: Start/End Interaction Events
  (Variables|Default|SetInteractor Interactor)
  (Default|ToggleInteractionWidget (Variables|Default|GetAC_Interactable) false)
  (CallFunction|OpenChest)
  (Input|SetIgnoreMoveInput (.As플레이어%20컨트롤러 (Utilities|Casting|CastToPlayerController (Variables|Default|GetInteractor))) true)
  (bind _returnvalue (Utilities|Time|SetTimerbyEvent (delegate Custom|Open%20Widget) 0.5))
  (Variables|Default|SetOpening%20Timer _returnvalue))

(event EventClientEndInteraction
  (bind _interactor (Variables|Default|GetInteractor))
  ;[0 1 0.01898 0.551] CLIENT: Start/End Interaction Events
  (Utilities|Time|ClearandInvalidateTimerbyHandle (Variables|Default|GetOpening%20Timer))
  (CallFunction|CloseChest)
  (Default|ToggleInteractionWidget (Variables|Default|GetAC_Interactable) true)
  (Utilities|IsValid _interactor
    (:Is%20Valid
      (Input|ResetIgnoreMoveInput (.As플레이어%20컨트롤러 (Utilities|Casting|CastToPlayerController _interactor)))
      (bind _widget (Class|DELETEBPIWidgetManager|DELETEGetActiveWidget(Message) (Variables|Default|GetInteractor)))
      (if (Utilities|Enum|Equal(Enum) _widget "Storage")
        (Class|DELETEBPIWidgetManager|DELETECloseActiveWidget(Message) (Variables|Default|GetInteractor))))))

(event EventInteraction
  (params (Interactor :type Actor%20Object%20Reference))
  ;[1 0 0.01436 0.248] SERVER: Start/End Interaction Events
  (Utilities|IsValid Interactor
    (:Is%20Valid
      (bind _output_get (Variables|Default|SetInteractor Interactor))
      (Actor|SetOwner _output_get)
      (CallFunction|ClientStartInteraction (Variables|Default|GetInteractor)))))

(event EventEndInteraction
  (params (Interactor :type Actor%20Object%20Reference))
  ;[1 0 0.01436 0.248] SERVER: Start/End Interaction Events
  (Utilities|IsValid Interactor
    (:Is%20Valid
      (bind _output_get (Variables|Default|SetInteractor Interactor))
      (Actor|SetOwner _output_get)
      (CallFunction|ClientEndInteraction))))

(fn ConstructionScript
  (|CallParentFunction))