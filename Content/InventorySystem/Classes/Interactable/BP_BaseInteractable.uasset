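; BP_BaseInteractable is a base interactable for the inventory system, with empty hooks for interaction, client start/end and game load.
; On Initialize it gives ACInteractable its area, widget and both meshes as highlightable objects.
; The construction script shows the skeletal mesh only when no static mesh is assigned.
; TryToTransferItems calls ServerTakeAllItems on the interactor's DELETE_AC_PlayerInventory component to take everything from an owner inventory.
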(event Custom|Client%20Start%20Interaction
  (params (Interactor :type Actor%20Object%20Reference))
  ;[0 0 0 0.227 22] Client Events
)

(event Custom|Client%20End%20Interaction
  ;[0 0 0 0.227 22] Client Events
)

(event EventInteraction
  (params (Interactor :type Actor%20Object%20Reference))
  ;[0 0 0 0.227 22] On Interaction
)

(event EventEndInteraction
  (params (Interactor :type Actor%20Object%20Reference))
  ;[0 0 0 0.227 22] On End Interaction
)

(event EventInitialize
  ;[0 0 0 0.227 22] On Initialize
  (Default|SetupInteractableReferences (Variables|Default|GetAC_Interactable) (Variables|Default|GetInteractableArea) (Variables|Default|GetInteractionWidget) (Utilities|Set|MakeSet (Variables|Default|GetStaticMesh) (Variables|Default|GetSkeletalMesh))))

(event EventRemoveInteraction
  ;[0 0 0 0.227 22] On Remove Interaction
)

(event EventGameLoad
  ;[0 0 0 0.227 22] On Game Load
)

(fn ConstructionScript
  (Rendering|SetVisibility (Variables|Default|GetSkeletalMesh) (select (Utilities|IsValid (Variables|/Script/Engine.StaticMeshComponent|GetStaticMesh (Variables|Default|GetStaticMesh))) false true) false))

(fn TrytoTransferItems
  (params (Interactor :type Actor%20Object%20Reference) (Owner%20Inventory :type DELETE%20AC%20Inventory%20Core%20Object%20Reference))
  (bind _returnvalue (Actor|GetComponentbyClass Interactor "/Game/InventorySystem/Blueprints/Components/DELETE_AC_PlayerInventory.DELETE_AC_PlayerInventory_C"))
  (Utilities|IsValid Owner%20Inventory
    (:Is%20Valid
      (Utilities|IsValid _returnvalue
        (:Is%20Valid
          (Default|ServerTakeAllItems _returnvalue Owner%20Inventory))))))