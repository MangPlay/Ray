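; BP_RayPlayerController is the player controller that routes input for inventory, loot and consumable pockets.
; Pocket and take-all-loot actions reach ConsumableBuffsComponent and PlayerInventory only while no main widget is open, whereas inventory toggle and widget close always pass through.
; It detects gamepad versus mouse from key presses and mouse axes, notifying the inventory widget controller of mode and focus changes.
; The Interaction input currently triggers no action.
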(event EventBeginPlay)

(event EventTick
  (params (DeltaSeconds :type Float%20%28single-precision%29)))

(event Input|ActionEvents|InputActionCloseWidget
  (params (Key :type Key%20Structure))
  ;[0 0.7454 0.4179 0.298 24] Main Inputs
  (:Pressed
    (Class|InventoryWidgetController|InputCloseWidget (Class|WidgetSystemLibrary|GetInventoryWidgetController))))

(event Input|ActionEvents|InputActionInteraction
  (params (Key :type Key%20Structure))
  ;[0 0.7454 0.4179 0.298 24] Main Inputs
  (:Pressed
    (if (CallFunction|IsAnyMainWidgetOpen)
      _)))

(event Input|ActionEvents|InputActionInventory
  (params (Key :type Key%20Structure))
  ;[0 0.7454 0.4179 0.298 24] Main Inputs
  (:Pressed
    (Class|PlayerInventoryComponent|InputInventory (Variables|Default|GetPlayerInventory))))

(event Input|ActionEvents|InputActionTakeAllLoot
  (params (Key :type Key%20Structure))
  ;[0 0.7454 0.4179 0.298 24] Main Inputs
  (:Pressed
    (if (not (CallFunction|IsAnyMainWidgetOpen))
      (Class|PlayerInventoryComponent|InputTakeAll (Variables|Default|GetPlayerInventory)))))

(event Input|ActionEvents|InputActionUsePocket1
  (params (Key :type Key%20Structure))
  ;[0 0.7454 0.4179 0.298] Pocket Inputs
  (:Released
    (if (not (CallFunction|IsAnyMainWidgetOpen))
      (Class|ConsumableBuffsComponent|OnUsePocket1 (Variables|Default|GetConsumableBuffsComponent)))))

(event Input|ActionEvents|InputActionUsePocket2
  (params (Key :type Key%20Structure))
  ;[0 0.7454 0.4179 0.298] Pocket Inputs
  (:Released
    (if (not (CallFunction|IsAnyMainWidgetOpen))
      (Class|ConsumableBuffsComponent|OnUsePocket2 (Variables|Default|GetConsumableBuffsComponent)))))

(event Input|ActionEvents|InputActionUsePocket3
  (params (Key :type Key%20Structure))
  ;[0 0.7454 0.4179 0.298] Pocket Inputs
  (:Released
    (if (not (CallFunction|IsAnyMainWidgetOpen))
      (Class|ConsumableBuffsComponent|OnUsePocket3 (Variables|Default|GetConsumableBuffsComponent)))))

(event Input|ActionEvents|InputActionUsePocket4
  (params (Key :type Key%20Structure))
  ;[0 0.7454 0.4179 0.298] Pocket Inputs
  (:Released
    (if (not (CallFunction|IsAnyMainWidgetOpen))
      (Class|ConsumableBuffsComponent|OnUsePocket4 (Variables|Default|GetConsumableBuffsComponent)))))

(fn ConstructionScript)

(fn IsAnyMainWidgetOpen
  (if (Utilities|Enum|NotEqual(Enum) (Variables|/Script/Ray.InventoryWidgetController|GetActiveWidget (Class|WidgetSystemLibrary|GetInventoryWidgetController)) "None")
    (return true)
    (else
      (return false))))

(fn DELETEGetRPGInventoryController
  (return 0))

(event EventSetCurrentlyFocusedWidget
  (params (Widget :type EWidgetType%20Enum :default "None"))
  (bind _returnvalue (Class|WidgetSystemLibrary|GetInventoryWidgetController))
  ;[0.01033 0.01033 0.01033 0.2196] Set Currently Focused Widget
  (if (Utilities|Enum|NotEqual(Enum) Widget (Variables|/Script/Ray.InventoryWidgetController|GetFocusedWidget (Class|WidgetSystemLibrary|GetInventoryWidgetController)))
    (Variables|/Script/Ray.InventoryWidgetController|SetFocusedWidget _returnvalue Widget)
    (Default|CallOnFocusedNewWidget _returnvalue)))

(event EventSetGamepadControls
  (params (IsGamepad :type Boolean))
  ;[0.01033 0.01033 0.01033 0.2196] Toggle Gamepad Controls
  (if (!= IsGamepad (Variables|Default|GetbGamepadControls))
    (bind _output_get (Variables|Default|SetbGamepadControls IsGamepad))
    (Default|CallOnGamepadToggled (Class|WidgetSystemLibrary|GetInventoryWidgetController) _output_get)
    (if (Variables|Default|GetbGamepadControls)
      (Class|PlayerController|SetMouseLocation))))

(event Input|MouseEvents|MouseX
  (params (AxisValue :type Float%20%28single-precision%29))
  ;[0.01033 0.01033 0.01033 0.2196] Check for Mouse Axis
  (if (or (!= AxisValue 0.0) (!= (stale Input|MouseEvents|MouseY AxisValue) 0.0))
    (CallFunction|SetGamepadControls false)))

(event Input|MouseEvents|MouseY
  (params (AxisValue :type Float%20%28single-precision%29))
  ;[0.01033 0.01033 0.01033 0.2196] Check for Mouse Axis
  (if (or (!= (stale Input|MouseEvents|MouseX AxisValue) 0.0) (!= AxisValue 0.0))
    (CallFunction|SetGamepadControls false)))

(event Input|KeyboardEvents|AnyKey
  (params (Key :type Key%20Structure :default "None"))
  ;[0.01033 0.01033 0.01033 0.2196] Check for Gamepad
  (:Pressed
    (CallFunction|SetGamepadControls (Class|KismetInputLibrary|KeyIsGamepadKey Key))))

(fn GetCurrentlyFocusedWidget
  (return (Variables|/Script/Ray.InventoryWidgetController|GetFocusedWidget (Class|WidgetSystemLibrary|GetInventoryWidgetController))))

(fn GetInventoryController
  (return self))

(fn IsUsingGamepad?
  (return (Variables|Default|GetbGamepadControls)))