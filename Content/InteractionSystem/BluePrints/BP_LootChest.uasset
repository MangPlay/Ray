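; BP_LootChest is an interactable chest that hands its inventory items to the interacting pawn.
; It registers its attach, marker and highlight components, and binds to InteractionTargetComponent begin/end events, making the interactor its owner.
; If ShowLootBar is on, client events play the open/close animations and toggle the loot bar widget.
; Otherwise, interaction skips the UI and animation, calling ServerTakeAllItems on the interactor's PlayerInventoryComponent to take everything.
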(event Custom|Open%20Chest
  ;[1 0.5038 0 0.426] CLIENT: Open/Close Chest
  (if (not (Variables|Default|GetIsOpen))
    (Components|Animation|PlayAnimation (Variables|Default|GetInteractionMesh) 0 false)
    (Variables|Default|SetIsOpen true)))

(event Custom|Close%20Chest
  ;[1 0.5038 0 0.426] CLIENT: Open/Close Chest
  (if (Variables|Default|GetIsOpen)
    (Components|Animation|PlayAnimation (Variables|Default|GetInteractionMesh) 0 false)
    (Variables|Default|SetIsOpen false)))

(event Custom|Interaction%20Begin
  (params (InteractorPawn :type Pawn%20Object%20Reference))
  ;[1 0 0.01436 0.248] 서버: 상호작용 이벤트 시작/종료
  (Utilities|IsValid InteractorPawn
    (:Is%20Valid
      (bind _output_get (Variables|Default|SetInteractor InteractorPawn))
      (Actor|SetOwner _output_get)
      (if (not (Variables|/Script/Ray.InventoryWidgetController|GetbShowLootBar (Class|WidgetSystemLibrary|GetInventoryWidgetController)))
        ;;[1 0.103 0 0.305] Bypass Opening LootBar
        (CallFunction|TrytoTransferItems (Variables|Default|GetInteractor) (Variables|Default|GetInventoryCore))
        (else
          (CallFunction|ClientStartInteraction (Variables|Default|GetInteractor)))))))

(event Custom|Interaction%20End
  (params (InteractionResult :type EInteractionResult%20Enum :default "Completed") (InteractorPawn :type Pawn%20Object%20Reference))
  ;[1 0 0.01436 0.248] 서버: 상호작용 이벤트 시작/종료
  (Utilities|IsValid InteractorPawn
    (:Is%20Valid
      (bind _output_get (Variables|Default|SetInteractor InteractorPawn))
      (Actor|SetOwner _output_get)
      (if (Variables|/Script/Ray.InventoryWidgetController|GetbShowLootBar (Class|WidgetSystemLibrary|GetInventoryWidgetController))
        (CallFunction|ClientEndInteraction)))))

(event Custom|ClientStartInteraction
  (params (Interactor :type Actor%20Object%20Reference))
  ;[0 1 0.01898 0.551] CLIENT: Start/End Interaction Events
  (CallFunction|OpenChest)
  (Class|InventoryWidgetController|OpenLootBarWidget (Class|WidgetSystemLibrary|GetInventoryWidgetController)))

(event Custom|ClientEndInteraction
  ;[0 1 0.01898 0.551] CLIENT: Start/End Interaction Events
  (CallFunction|CloseChest)
  (Utilities|IsValid (Variables|Default|GetInteractor)
    (:Is%20Valid
      (Class|InventoryWidgetController|CloseLootBarWidget (Class|WidgetSystemLibrary|GetInventoryWidgetController)))))

(event EventBeginPlay
  ;[1 0.3281 0] Begin Play Event
  (EventDispatchers|BindEventtoOnInteractionBegin (Variables|Default|GetInteractionTargetComponent) (delegate Custom|Interaction%20Begin))
  (EventDispatchers|BindEventtoOnInteractionEnd (Variables|Default|GetInteractionTargetComponent) (delegate Custom|Interaction%20End)))

(event Collision|EventActorBeginOverlap
  (params (OtherActor :type Actor%20Object%20Reference)))

(event EventInitializeInteractable
  (Class|InterfaceInteractable|SetupOverlapAttachComponent(Message) self (Variables|Default|GetScene))
  (Class|InterfaceInteractable|SetupMarkerTargetComponent(Message) self (Variables|Default|GetMarkerTarget))
  (Class|InterfaceInteractable|SetupHighlightedComponents(Message) self (Utilities|Array|MakeArray (Variables|Default|GetInteractionMesh))))

(fn ConstructionScript)

(fn TrytoTransferItems
  (params (Interactor :type Actor%20Object%20Reference) (Owner%20Inventory :type Inventory%20Core%20Object%20Reference))
  (bind _returnvalue (Actor|GetComponentbyClass Interactor "/Script/Ray.PlayerInventoryComponent"))
  (Utilities|IsValid Owner%20Inventory
    (:Is%20Valid
      (Utilities|IsValid _returnvalue
        (:Is%20Valid
          (Class|PlayerInventoryComponent|ServerTakeAllItems _returnvalue Owner%20Inventory))))))